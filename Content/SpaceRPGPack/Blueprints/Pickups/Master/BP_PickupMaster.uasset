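; Master pickup Blueprint that flies to the player when approached, with child classes overriding CustomOnPickupEvent for the reward.
; A pawn entering SphereTrigger removes it and starts a timeline that pulls the shrinking mesh toward player 0, then destroys the actor.
; The first pawn touching the mesh fires the event, 2D sound and Niagara burst.
; PickupColor tints that burst and the construction-time dynamic material.
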(event `self.PickupMesh.OnComponentBeginOverlap`
  (params (OverlappedComponent :type "PrimitiveComponent Object Reference") (OtherActor :type "Actor Object Reference") (OtherComp :type "PrimitiveComponent Object Reference") (OtherBodyIndex :type Integer) (bFromSweep :type Boolean) (SweepResult :type "HitResult Structure (by ref)"))
  ;[0.1441 0.004391 0.004025] Event Actor Begin Overlap  - Effects and destroy
  ;;[1 1 1] Check if it is the player, if so, play collected sound and visual effect, then destroy self.
  (cast `Pawn` OtherActor)
  (`/Engine/EditorBlueprintResources/StandardMacros.DoOnce` false
    (:`Completed`
      (`self.Custom On Pickup Event` OtherActor)
      (`GameplayStatics.PlaySound2D` (`self.Sound for Collected`) 1.0 1.0 0.0 null null)
      (bind _returnvalue (`NiagaraFunctionLibrary.SpawnSystemAtLocation` (`self.System for Collected`) (`self.K2_GetActorLocation`)))
      (`FXSystemComponent.SetColorParameter` _returnvalue "Color" (`self.Pickup Color`))
      (`PrimitiveComponent.SetCollisionResponseToChannel` (`self.PickupMesh`) "ECC_Pawn" "ECR_Ignore"))))

(event `self.Sphere Trigger.OnComponentBeginOverlap`
  (params (OverlappedComponent :type "PrimitiveComponent Object Reference") (OtherActor :type "Actor Object Reference") (OtherComp :type "PrimitiveComponent Object Reference") (OtherBodyIndex :type Integer) (bFromSweep :type Boolean) (SweepResult :type "HitResult Structure (by ref)"))
  ;[0.1441 0.004391 0.004025] On Component Overlap (Sphere Trigger) - Player Attraction
  (cast `Pawn` OtherActor)
  (`ActorComponent.K2_DestroyComponent` (`self.Sphere Trigger`))
  (bind (_direction _pickup_movement) (`Timeline|Timeline_0` :!via `PlayFromStart`)
    (:`Update`
      (`SceneComponent.K2_SetWorldLocation` (`self.PickupMesh`) (`KismetMathLibrary.VLerp` (`SceneComponent.K2_GetComponentLocation` (`self.PickupMesh`)) (+ (`self.K2_GetActorLocation` (`GameplayStatics.GetPlayerPawn` 0)) (0.0 0.0 40.0)) _pickup_movement) false false)
      (`SceneComponent.SetRelativeScale3D` (`self.PickupMesh`) (`KismetMathLibrary.VLerp` (`SceneComponent.RelativeScale3D` (`self.PickupMesh`)) (0.01 0.01 0.01) _pickup_movement)))
    (:`Finished`
      (`self.K2_DestroyActor`))))

(event `Custom On Pickup Event`
  (params (`Other Actor` :type "Actor Object Reference"))
  ;[0.1441 0.004391 0.004025] Custom Event On Pickup -
)

(fn `UserConstructionScript`
  (bind _returnvalue (`PrimitiveComponent.CreateDynamicMaterialInstance` (`self.Sphere`) 0 "/Game/SpaceRPGPack/Materials/MasterMaterials/M_EnergyNEffect.M_EnergyNEffect" "None"))
  (`MaterialInstanceDynamic.SetVectorParameterValue` _returnvalue "Base Color" (`self.Pickup Color`)))