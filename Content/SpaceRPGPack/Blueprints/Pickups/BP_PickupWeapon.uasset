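; BP_PickupWeapon is a weapon pickup that awards a DT_Weapons entry to the actor that collects it.
; On construction it takes the row from its data handler, or a random one when RandomDrop is set.
; SetDropDisplay shows that weapon's name and color on the text render and overrides PickupColor before the parent construction runs.
; On pickup it sends the row name through BPI_Pickups to the other actor's components.
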(event `self.Custom On Pickup Event`
  (params (`Other Actor` :type "Actor Object Reference"))
  ;[0.1441 0.004391 0.004025] Custom Pickup Event - Match Row Name with the same name within "DT_Weapons", and the component will get the message to award the correct data.
  (message `/Game/SpaceRPGPack/Blueprints/Framework/Interfaces/BPI_Pickups.Weapon Interact` (`self.GetComponentsByInterface` `Other Actor` "/Game/SpaceRPGPack/Blueprints/Framework/Interfaces/BPI_Pickups.BPI_Pickups_C") (`self.Row Name`)))

(fn `Set Drop Display`
  (params (RowName :type Name))
  ;[0.1301 0.005605 0.2016] Set Drop Display - This is hard coded to use the "DT_Weapons" data table. We use it to display specific weapon names and colors on the pickup text render and the display material.
  (bind _returnvalue (`|GetDataTableRow` "/Game/SpaceRPGPack/Blueprints/Framework/DataTables/DT_Weapons.DT_Weapons" RowName)
    (:`then`
      (bind ((`WeaponName_23_29942F94467AD7E6C12EBE9C16FDED39` _weaponname) (`EffectSystem_52_D326E29B4F70F7CEF3D9E0960510F30F` _effectsystem) (`WeaponColor_46_CFFCA00942E8CE544ED6AFBDE4AA0E30` _weaponcolor)) (break `/Game/SpaceRPGPack/Blueprints/Framework/Structures/S_Weapons` _returnvalue))
      (`TextRenderComponent.K2_SetText` (`self.TextRender`) _weaponname)
      (set `self.Pickup Color` _weaponcolor) ; We override the color set in the defaults with the one associated with the weapon.
      (`TextRenderComponent.SetTextRenderColor` (`self.TextRender`) (`KismetMathLibrary.Conv_LinearColorToColor` _weaponcolor)))))

(fn `UserConstructionScript`
  (bind (_datatable _rowname) (break `DataTableRowHandle` (`self.Data Handler`)))
  ;[0.1301 0.005605 0.2016] Construct - We check the selected weapon for its name and the color associated with it then call the function to set this display.
  (if (`self.Random Drop?`)
    (bind _outrownames (`DataTableFunctionLibrary.GetDataTableRowNames` _datatable))
    (set `self.Row Name` (`KismetArrayLibrary.Array_Random` _outrownames))
    (else
      (set `self.Row Name` _rowname)))
  (`self.Set Drop Display` (`self.Row Name`))
  (`parent.UserConstructionScript`))