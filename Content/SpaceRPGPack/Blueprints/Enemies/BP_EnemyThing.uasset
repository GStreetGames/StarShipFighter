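; BP_EnemyThing is an enemy actor with a health widget, optional shields and a weapon system component.
; Its range trigger radius sets projectile range, and overlap by a BP_Ship_Base unpauses or pauses the weapon's Fire timer, which starts paused.
; Damage turns the health widget toward the player camera and briefly flashes shield opacity or hull emissive, using dynamic materials cached in the construction script.
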(event `self.ReceiveBeginPlay`
  ;[1 1 1] On Begin Play -
  (`parent.ReceiveBeginPlay`)
  (`|ExecutionSequence`
    (:`then_0`
      (bind _aswbp_enemy_health (cast `/Game/SpaceRPGPack/Widgets/WBP_EnemyHealth` (`WidgetComponent.GetUserWidgetObject` (`self.Health Widget`))))
      (set `/Game/SpaceRPGPack/Widgets/WBP_EnemyHealth.Enemy` self _aswbp_enemy_health)
      (set `/Game/SpaceRPGPack/Blueprints/Components/AC_EnemyWeaponSystem.Projectile Range` (`SphereComponent.SphereRadius` (`self.Enemy Range Trigger`)) (`self.AC_EnemyWeaponSystem`)))
    (:`then_1`
      (`MaterialInstanceDynamic.SetVectorParameterValue` (`self.Enemy Material`) "Emissive Color" (`self.Hit Effect Color`)))
    (:`then_2`
      ;;[1 1 1] Pause the weapon system component for now
      (`KismetSystemLibrary.K2_PauseTimer` (`self.AC_EnemyWeaponSystem`) "Fire"))))

(event `self.Enemy Range Trigger.OnComponentBeginOverlap`
  (params (OverlappedComponent :type "PrimitiveComponent Object Reference") (OtherActor :type "Actor Object Reference") (OtherComp :type "PrimitiveComponent Object Reference") (OtherBodyIndex :type Integer) (bFromSweep :type Boolean) (SweepResult :type "HitResult Structure (by ref)"))
  ;[1 1 1] Activate Triggering
  (cast `/Game/SpaceRPGPack/Blueprints/BP_Ship_Base` OtherActor)
  (`KismetSystemLibrary.K2_UnPauseTimer` (`self.AC_EnemyWeaponSystem`) "Fire"))

(event `self.ReceiveAnyDamage`
  (params (Damage :type "Float (single-precision)") (DamageType :type "DamageType Object Reference") (InstigatedBy :type "Controller Object Reference") (DamageCauser :type "Actor Object Reference"))
  (bind _ac_health (`self.AC_Health`))
  ;[1 1 1] Event Any Damage -
  (`self.Update Direction`)
  (if (and (`/Game/SpaceRPGPack/Blueprints/Components/AC_Health.Has Shield?` _ac_health) (> (`/Game/SpaceRPGPack/Blueprints/Components/AC_Health.Shields` _ac_health) 0.0))
    (`MaterialInstanceDynamic.SetScalarParameterValue` (`self.Shields Material`) "Overall Opacity" 1.0)
    (`KismetSystemLibrary.Delay` 0.3)
    (`MaterialInstanceDynamic.SetScalarParameterValue` (`self.Shields Material`) "Overall Opacity" 0.0)
    (else
      (`MaterialInstanceDynamic.SetScalarParameterValue` (`self.Enemy Material`) "Emissive Strength" 1.0)
      (`KismetSystemLibrary.Delay` 0.1)
      (`MaterialInstanceDynamic.SetScalarParameterValue` (`self.Enemy Material`) "Emissive Strength" 0.0))))

(event `self.Enemy Range Trigger.OnComponentEndOverlap`
  (params (OverlappedComponent :type "PrimitiveComponent Object Reference") (OtherActor :type "Actor Object Reference") (OtherComp :type "PrimitiveComponent Object Reference") (OtherBodyIndex :type Integer))
  ;[1 1 1] Activate Triggering
  (cast `/Game/SpaceRPGPack/Blueprints/BP_Ship_Base` OtherActor)
  (`KismetSystemLibrary.K2_PauseTimer` (`self.AC_EnemyWeaponSystem`) "Fire"))

(fn `Update Direction`
  (bind _health_widget (`self.Health Widget`))
  (`SceneComponent.K2_SetWorldRotation` _health_widget (`KismetMathLibrary.FindLookAtRotation` (`SceneComponent.K2_GetComponentLocation` _health_widget) (`SceneComponent.K2_GetComponentLocation` (`Actor.RootComponent` (`GameplayStatics.GetPlayerCameraManager` 0)))) false false))

(fn `UserConstructionScript`
  (bind _shields (`self.Shields`))
  (bind _enemymesh (`self.EnemyMesh`))
  (`parent.UserConstructionScript`)
  ;[1 1 1] Get and cache the material thats applied to the Enemy Mesh.
  (bind _returnvalue (`PrimitiveComponent.CreateDynamicMaterialInstance` _enemymesh 0 (`PrimitiveComponent.GetMaterial` _enemymesh 0) "None"))
  (set `self.Enemy Material` _returnvalue)
  ;[1 1 1] Get and cache the material thats applied to the Shields Mesh.
  (bind _returnvalue_2 (`PrimitiveComponent.CreateDynamicMaterialInstance` _shields 0 (`PrimitiveComponent.GetMaterial` _shields 0) "None"))
  (set `self.Shields Material` _returnvalue_2))