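; Enemy projectile actor that flies at a set speed, damages whatever its mesh hits, then destroys itself.
; The construction script feeds the speed into the projectile movement and derives lifespan from range divided by speed, so range caps travel distance.
; It also creates a dynamic material instance on the mesh to apply the two configurable projectile colors.
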(event `self.Projectile Mesh.OnComponentHit`
  (params (HitComponent :type "PrimitiveComponent Object Reference") (OtherActor :type "Actor Object Reference") (OtherComp :type "PrimitiveComponent Object Reference") (NormalImpulse :type "Vector Structure") (Hit :type "HitResult Structure (by ref)"))
  (`GameplayStatics.ApplyDamage` OtherActor (`self.Projectile Damage`) null self (`self.Damage Type Class`))
  (`self.K2_DestroyActor`))

(fn `UserConstructionScript`
  (bind _projectile_mesh (`self.Projectile Mesh`))
  (bind _projectilemovement (`self.ProjectileMovement`))
  (bind _output_get (set `ProjectileMovementComponent.MaxSpeed` (`self.Projectile Speed`) _projectilemovement))
  (set `ProjectileMovementComponent.InitialSpeed` _output_get _projectilemovement)
  (`self.SetLifeSpan` self (/ (`self.Projectile Range`) (`ProjectileMovementComponent.InitialSpeed` _projectilemovement)))
  (bind _returnvalue (`PrimitiveComponent.CreateDynamicMaterialInstance` _projectile_mesh 0 (`PrimitiveComponent.GetMaterial` _projectile_mesh 0) "None"))
  (bind _output_get_2 (set `self.material` _returnvalue))
  (`MaterialInstanceDynamic.SetVectorParameterValue` _output_get_2 "Base Color" (`self.Projectile Color`))
  (`MaterialInstanceDynamic.SetVectorParameterValue` (`self.material`) "Second Color" (`self.Projectile Color 2`)))