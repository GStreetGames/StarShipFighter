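; BP_Meteoroid is a damageable meteoroid enemy with randomized looks and tumble.
; Its construction script picks a random rotation rate, mesh and material, makes the material dynamic, and applies RandomHealth as max health when FieldSpawned.
; On BeginPlay it matches the ACExplodeOnDestroy effect scale to the mesh's world scale.
; Taking damage briefly raises the material's emissive strength as a hit blink.
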(event `self.ReceiveBeginPlay`
  (`parent.ReceiveBeginPlay`)
  ;[1 1 1] Set particle effect scale to match the mesh size of the asteroid
  (bind _output_get (set `self.World Scale Holder` (`SceneComponent.K2_GetComponentScale` (`self.EnemyMesh`))))
  (set `/Game/SpaceRPGPack/Blueprints/Components/AC_ExplodeOnDestroy.System Effect Scale` _output_get (`self.AC_ExplodeOnDestroy`)))

(event `self.ReceiveAnyDamage`
  (params (Damage :type "Float (single-precision)") (DamageType :type "DamageType Object Reference") (InstigatedBy :type "Controller Object Reference") (DamageCauser :type "Actor Object Reference"))
  (bind _dynamic_material (`self.Dynamic Material`))
  ;[1 1 1] Hit blinking effect
  (`MaterialInstanceDynamic.SetScalarParameterValue` _dynamic_material "Emissive Strength" 1.0)
  (`KismetSystemLibrary.Delay` 0.18)
  (`MaterialInstanceDynamic.SetScalarParameterValue` _dynamic_material "Emissive Strength" 0.0))

(fn `UserConstructionScript`
  (bind _outitem (`KismetArrayLibrary.Array_Random` (`self.Material Choices`)))
  (`parent.UserConstructionScript`)
  ;[1 1 1] Randomly Set the Rotation
  (set `RotatingMovementComponent.RotationRate` (`KismetMathLibrary.MakeRotator` (`KismetMathLibrary.RandomFloatInRange` 0.7 19.0) (`KismetMathLibrary.RandomFloatInRange` 0.3 17.0) (`KismetMathLibrary.RandomFloatInRange` 0.5 15.0)) (`self.RotatingMovement`))
  ;[1 1 1] Randomly set the applied material
  (`PrimitiveComponent.SetMaterial` (`self.EnemyMesh`) 0 _outitem)
  ;[1 1 1] Make the set material a dynamic reference.
  (bind _returnvalue (`PrimitiveComponent.CreateDynamicMaterialInstance` (`self.EnemyMesh`) 0 _outitem "None"))
  (set `self.Dynamic Material` _returnvalue)
  ;[1 1 1] Randomly set the mesh
  (`StaticMeshComponent.SetStaticMesh` (`self.EnemyMesh`) (`KismetArrayLibrary.Array_Random` (`self.Mesh Choices`)))
  ;[1 1 1] Random Health Generation
  (if (`self.Field Spawned?`)
    (set `/Game/SpaceRPGPack/Blueprints/Components/AC_Health.Max Health` (`self.Random Health`) (`self.AC_Health`))))