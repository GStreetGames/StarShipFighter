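; Destructible asteroid actor that plays its explosion as soon as it spawns.
; BeginPlay spawns one of three random Niagara explosions using the Geometry Collection's scale, plus a BP_StressField_A field actor at the collection's transform.
; It plays one of three random explosion sounds in 2D, then destroys the field and itself in the same execution chain, with no delay.
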(event `self.ReceiveBeginPlay`
  (`NiagaraFunctionLibrary.SpawnSystemAtLocation` (select `int` (`KismetMathLibrary.RandomIntegerInRange` 0 2) :`0` "/Game/SpaceRPGPack/Effects/NS_Asteroid_Explosion_01.NS_Asteroid_Explosion_01" :`1` "/Game/SpaceRPGPack/Effects/NS_Asteroid_Explosion_02.NS_Asteroid_Explosion_02" :`2` "/Game/SpaceRPGPack/Effects/NS_Asteroid_Explosion_03.NS_Asteroid_Explosion_03" :!type "NiagaraSystem Object Reference") (`self.K2_GetActorLocation`) (struct) (`SceneComponent.K2_GetComponentScale` (`self.GeometryCollectionComponent`)))
  (bind _returnvalue (`|SpawnActorFromClass` "/Game/SpaceRPGPack/Blueprints/Environment/BP_StressField_A.BP_StressField_A_C" (`SceneComponent.K2_GetComponentToWorld` (`self.GeometryCollectionComponent`)) "AlwaysSpawn" "OverrideRootScale" null null))
  (`GameplayStatics.PlaySound2D` (select `int` (`KismetMathLibrary.RandomIntegerInRange` 0 2) :`0` "/Game/SpaceRPGPack/Audio/CUE/CUE_Explode_00.CUE_Explode_00" :`1` "/Game/SpaceRPGPack/Audio/CUE/CUE_Explode_01.CUE_Explode_01" :`2` "/Game/SpaceRPGPack/Audio/CUE/CUE_Explode_02.CUE_Explode_02" :!type "SoundBase Object Reference") 1.0 1.0 0.0 null null)
  (`self.K2_DestroyActor` _returnvalue)
  (`self.K2_DestroyActor`))

(fn `UserConstructionScript`)