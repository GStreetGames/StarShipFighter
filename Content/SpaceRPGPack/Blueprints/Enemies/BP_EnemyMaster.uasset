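; Base enemy Blueprint that shows visual feedback for status effects reported by its health component.
; BeginPlay creates dynamic ice and fire materials, which Frozen and Burning apply as mesh overlays with tuned intensity.
; Every status update, on or off, spawns a matching Niagara system at the mesh, including Stunned and Irradiated, which have no overlay.
; A separate NewMeshEvent adds an enlarged, collision-ignoring mesh copy with an ice material.
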(event `self.ReceiveBeginPlay`
  ;[0.1441 0.004391 0.004025] Event Begin Play -
  (bind _returnvalue (`KismetMaterialLibrary.CreateDynamicMaterialInstance` (`self.Ice Material`)))
  (set `self.Dynamic Ice` _returnvalue)
  (bind _returnvalue_2 (`KismetMaterialLibrary.CreateDynamicMaterialInstance` (`self.Fire Material`)))
  (set `self.Dynamic Fire` _returnvalue_2))

(event `New Mesh Event`
  (bind (_returnvalue_location _returnvalue_rotation _returnvalue_scale) (`KismetMathLibrary.BreakTransform` (`SceneComponent.GetRelativeTransform` (`self.EnemyMesh`))))
  ;[0.1441 0.004391 0.004025] New Mesh Event
  (bind _returnvalue (`AddComponent|NODE_AddStaticMeshComponent-0` :`bManualAttachment` true :`RelativeTransform` (`KismetMathLibrary.MakeTransform` _returnvalue_location _returnvalue_rotation (+ _returnvalue_scale (1.0 1.0 1.0)))))
  (`StaticMeshComponent.SetStaticMesh` _returnvalue (`StaticMeshComponent.StaticMesh` (`self.EnemyMesh`)))
  (`PrimitiveComponent.SetCollisionResponseToAllChannels` _returnvalue "ECR_Ignore")
  (`PrimitiveComponent.SetMaterial` _returnvalue 0 "/Game/SpaceRPGPack/DEMO/Materials/Epic/eFFECTS/M_Ice_Interactive.M_Ice_Interactive"))

(event `self.AC_Health.On Updated Status Effect`
  (params (`Status Type` :type "/Game/SpaceRPGPack/Blueprints/Framework/Enumerations/E_StatusEffects Enum" :default "NewEnumerator0") (`Activated?` :type Boolean))
  ;[0.1441 0.004391 0.004025] Status Effect Event -
  (switch `/Game/SpaceRPGPack/Blueprints/Framework/Enumerations/E_StatusEffects` `Status Type`
    (:`NewEnumerator0`
      (`MeshComponent.SetOverlayMaterial` (`self.EnemyMesh`) (select `bool` `Activated?` :`true` (`self.Dynamic Ice`) :!type "MaterialInterface Object Reference"))
      (`MaterialInstanceDynamic.SetScalarParameterValue` (`self.Dynamic Ice`) "Coldness" 0.1))
    (:`NewEnumerator1`
      (`MeshComponent.SetOverlayMaterial` (`self.EnemyMesh`) (select `bool` `Activated?` :`true` (`self.Dynamic Fire`) :!type "MaterialInterface Object Reference"))
      (`MaterialInstanceDynamic.SetScalarParameterValue` (`self.Dynamic Fire`) "Heat" 0.5))
    (:`NewEnumerator2`
      _)
    (:`NewEnumerator3`
      _))
  (`self.Niagara Damage Effect` (select `/Game/SpaceRPGPack/Blueprints/Framework/Enumerations/E_StatusEffects` `Status Type` :`NewEnumerator0` (`self.Frozen`) :`NewEnumerator1` (`self.Burning`) :`NewEnumerator2` (`self.Stunned`) :`NewEnumerator3` (`self.Irradiated`))))

(fn `Niagara Damage Effect`
  (params (SystemTemplate :type "NiagaraSystem Object Reference"))
  (returns (ReturnValue :type "NiagaraComponent Object Reference"))
  (bind (_returnvalue_location _returnvalue_rotation _returnvalue_scale) (`KismetMathLibrary.BreakTransform` (`SceneComponent.K2_GetComponentToWorld` (`self.EnemyMesh`))))
  (bind _returnvalue (`NiagaraFunctionLibrary.SpawnSystemAtLocation` SystemTemplate _returnvalue_location _returnvalue_rotation _returnvalue_scale))
  (return _returnvalue))

(fn `UserConstructionScript`)