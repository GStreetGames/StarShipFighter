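; BP_Missiles is a player missile projectile that homes in on a targeted enemy.
; On BeginPlay it takes the HUD's HitActor, stores it as the initial target if it is a BP_EnemyMaster, and sets the projectile movement to home on that actor's scene component.
; The construction script runs the parent's, then scales the hit explosion effect by the projectile multiplier, with a size clamp.
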(event `self.ReceiveBeginPlay`
  ;[1 1 1] Begin Play -
  (bind _asbp_hud (cast `/Game/SpaceRPGPack/Blueprints/Framework/BP_HUD` (`PlayerController.GetHUD` (`GameplayStatics.GetPlayerController` 0))))
  (bind _output_get (set `self.Hit Actor` (`/Game/SpaceRPGPack/Blueprints/Framework/BP_HUD.Hit Actor` _asbp_hud)))
  (`/Engine/EditorBlueprintResources/StandardMacros.IsValid` _output_get
    (:`Is Valid`
      (bind _asbp_enemy_master (cast `/Game/SpaceRPGPack/Blueprints/Enemies/BP_EnemyMaster` (`self.Hit Actor`)))
      (bind _output_get_2 (set `self.Initial Target` _asbp_enemy_master))
      (`/Engine/EditorBlueprintResources/StandardMacros.IsValid` _output_get_2
        (:`Is Valid`
          (`self.Lockon Target`))))))

(event `Lockon Target`
  (bind _projectilemovement (`self.ProjectileMovement`))
  ;[1 1 1] Lockon Custom Event -
  (set `ProjectileMovementComponent.HomingTargetComponent` (`self.GetComponentByClass` (`self.Initial Target`) "/Script/Engine.SceneComponent") _projectilemovement)
  (set `ProjectileMovementComponent.bIsHomingProjectile` true _projectilemovement))

(fn `UserConstructionScript`
  ;[0.154 0 0.2042] On Construct -
  (`parent.UserConstructionScript`)
  ;;[1 1 1] Expand explosion effect radius based on projectile multiplier
  (set `self.Hit Effect Scale` (`KismetMathLibrary.Vector_ClampSizeMax` (* (2.2 2.2 2.2) (`self.Projectile Multiplier`)) 16.0)))