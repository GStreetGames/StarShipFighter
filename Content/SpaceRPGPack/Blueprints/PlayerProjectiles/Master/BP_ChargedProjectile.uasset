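; Charged player projectile Blueprint that grows while charging and scales its damage by the charge level at fire time.
; A timeline started on BeginPlay drives the charge amount, which scales the actor up toward a maximum charge scale.
; Firing stops the timeline, multiplies damage by the charge, and activates projectile movement along the weapon component's forward vector.
; The charge amount is also exposed as a damage multiplier.
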(event `self.ReceiveBeginPlay`
  (`parent.ReceiveBeginPlay`)
  (bind (_direction _charge_amount) (`Timeline|Charge Timeline` :!label _label)
    (:`Update`
      (bind _output_get (set `self.Charge Amount` _charge_amount))
      (bind _output_get_2 (set `self.Charge` (`KismetMathLibrary.Conv_DoubleToVector` (* _output_get (`self.Max Charge Scale`)))))
      (`self.SetActorScale3D` _output_get_2))))

(event `self.Fire`
  (params (`Weapon Component` :type "SceneComponent Object Reference"))
  (bind _projectilemovement (`self.ProjectileMovement`))
  (`parent.Fire` `Weapon Component`)
  (`MovementComponent.SetUpdatedComponent` (`self.ProjectileMovement`) (`self.ProjectileMesh`))
  (`ActorComponent.Activate` _projectilemovement true)
  (set `MovementComponent.Velocity` (* (`ProjectileMovementComponent.InitialSpeed` _projectilemovement) (`SceneComponent.GetForwardVector` `Weapon Component`)) (`self.ProjectileMovement`))
  (set `self.Projectile Damage` (* (`self.Projectile Damage`) (`self.Charge Amount`)))
  (goto _label :!via `Stop`))

(fn `Get Damage Multiplier`
  (returns (`Damage Multiplier` :type "Float (double-precision)"))
  (return (`self.Charge Amount`)))

(fn `UserConstructionScript`
  (`parent.UserConstructionScript`))