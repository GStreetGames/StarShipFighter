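; Master projectile for player weapons in the space RPG pack, with color, effects, speed, range and damage driven by variables.
; Construction clamps multiplier-scaled speed, BeginPlay tints the material and Niagara effect, and Fire derives lifespan from range over speed.
; Hits apply damage, notify asteroids through BPI_AsteroidDamage, spawn effects and destroy the projectile.
; On destruction, including expiry, explosive types deal radial damage and sphere-trace for asteroids within a multiplier-scaled radius.
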(event `self.ReceiveBeginPlay`
  (bind _projectilemesh (`self.ProjectileMesh`))
  ;[0.1441 0.004391 0.004025] Event Begin Play -
  ;;[1 1 1] Set the default material properties. (Default projectile material properties, just override begin play if your child has a different projectile material.)
  (bind _returnvalue (`PrimitiveComponent.CreateDynamicMaterialInstance` _projectilemesh 0 (`PrimitiveComponent.GetMaterial` _projectilemesh 0) "None"))
  (set `self.ProjectileMaterial` _returnvalue)
  (`MaterialInstanceDynamic.SetVectorParameterValue` (`self.ProjectileMaterial`) "Base Color" (`self.Projectile Color`))
  (`MaterialInstanceDynamic.SetVectorParameterValue` (`self.ProjectileMaterial`) "Second Color" (`self.Projectile Color 2`))
  ;;[1 1 1] Set the Niagara Effect System to the value coming from the data table.
  (`NiagaraComponent.SetAsset` (`self.Niagara`) (`self.Projectile Effect System`) true)
  ;;[1 1 1] Set the Projectile Effect System colors to the values we get from the data table.
  (`FXSystemComponent.SetColorParameter` (`self.Niagara`) "Color" (`self.Projectile Color`))
  (`FXSystemComponent.SetColorParameter` (`self.Niagara`) "Color 2" (`self.Projectile Color 2`)))

(event `Fire`
  (params (`Weapon Component` :type "SceneComponent Object Reference"))
  ;[0.1441 0.004391 0.004025] Fire Custom Event -
  ;;[1 1 1] We set life span based on range divided by speed.
  (`self.SetLifeSpan` (/ (`self.Projectile Range`) (`ProjectileMovementComponent.InitialSpeed` (`self.ProjectileMovement`)))))

(event `self.ProjectileMesh.OnComponentHit`
  (params (HitComponent :type "PrimitiveComponent Object Reference") (OtherActor :type "Actor Object Reference") (OtherComp :type "PrimitiveComponent Object Reference") (NormalImpulse :type "Vector Structure") (Hit :type "HitResult Structure (by ref)"))
  ;[1 1 1] On Component Hit -
  (set `self.Component Hit?` true)
  (bind _impactpoint (`self.Hit Damage` OtherActor Hit))
  (`self.Spawn Hit Effects` _impactpoint)
  (`self.K2_DestroyActor`))

(event `self.ReceiveDestroyed`
  (bind _returnvalue (`GameplayStatics.GetPlayerPawn` 0))
  (bind _returnvalue_2 (`SceneComponent.K2_GetComponentLocation` (`self.ProjectileMesh`)))
  ;[1 1 1] Event Destroyed -
  (if (== (`self.Damage Type Class`) "/Game/SpaceRPGPack/Blueprints/DamageTypes/DT_Explosive.DT_Explosive_C")
    (`GameplayStatics.ApplyRadialDamage` (`self.Projectile Damage`) (`SceneComponent.K2_GetComponentLocation` (`self.ProjectileMesh`)) (`self.Set Radius`) (`self.Damage Type Class`) (`|MakeArray` self _returnvalue :!type "Actor Object Reference") (`self.Instigator`) (`self.GetInstigatorController` _returnvalue) true "ECC_GameTraceChannel1")
    (if (not (`self.Component Hit?`))
      (`self.Spawn Hit Effects` (`SceneComponent.K2_GetComponentLocation` (`self.ProjectileMesh`))))
    (bind _outhits (`KismetSystemLibrary.SphereTraceMulti` _returnvalue_2 _returnvalue_2 (`self.Set Radius`) "TraceTypeQuery3"))
    (for _array_element _outhits
      (bind (_bblockinghit _binitialoverlap _time _distance _location _impactpoint _normal _impactnormal _physmat _hitactor _hitcomponent _hitbonename _bonename _hititem) (`GameplayStatics.BreakHitResult` _array_element))
      (if (`KismetSystemLibrary.DoesImplementInterface` _hitactor "/Game/SpaceRPGPack/Blueprints/Framework/Interfaces/BPI_AsteroidDamage.BPI_AsteroidDamage_C")
        (message `/Game/SpaceRPGPack/Blueprints/Framework/Interfaces/BPI_AsteroidDamage.Hit Asteroid` _hitactor _hitcomponent _hititem)))))

(fn `Get Damage Multiplier`
  (returns (`Damage Multiplier` :type "Float (double-precision)"))
  (return 1.0))

(fn `Hit Damage`
  (params (DamagedActor :type "Actor Object Reference") (Hit :type "HitResult Structure (by ref)"))
  (returns (ImpactPoint :type "Vector Structure"))
  (bind (_bblockinghit _binitialoverlap _time _distance _location _impactpoint _normal _impactnormal _physmat _hitactor _hitcomponent _hitbonename _bonename _hititem) (`GameplayStatics.BreakHitResult` Hit))
  (`GameplayStatics.ApplyDamage` DamagedActor (* (`self.Projectile Damage`) (`self.Get Damage Multiplier`)) (`self.GetInstigatorController`) (`self.Instigator`) (`self.Damage Type Class`))
  (if (`KismetSystemLibrary.DoesImplementInterface` _hitactor "/Game/SpaceRPGPack/Blueprints/Framework/Interfaces/BPI_AsteroidDamage.BPI_AsteroidDamage_C")
    (message `/Game/SpaceRPGPack/Blueprints/Framework/Interfaces/BPI_AsteroidDamage.Hit Asteroid` _hitactor _hitcomponent _hititem))
  (return _location))

(fn `Set Radius`
  (returns (ReturnValue :type "Float (double-precision)"))
  (return (`KismetMathLibrary.FClamp` (* 1600.0 (`self.Projectile Multiplier`)) 1600.0 5600.0)))

(fn `Spawn Hit Effects`
  (params (Location :type "Vector Structure"))
  (bind _hitsoundeffect (`self.HitSoundEffect`))
  (`/Engine/EditorBlueprintResources/StandardMacros.IsValid` (`self.Hit Effect System`)
    (:`Is Valid`
      (bind _returnvalue (`NiagaraFunctionLibrary.SpawnSystemAtLocation` (`self.Hit Effect System`) Location (struct) (`self.Hit Effect Scale`)))
      (`FXSystemComponent.SetColorParameter` _returnvalue "Color" (`self.Projectile Color`))
      (`FXSystemComponent.SetColorParameter` _returnvalue "Color 2" (`self.Projectile Color 2`)))
    (:`Is Not Valid`
      _))
  (`/Engine/EditorBlueprintResources/StandardMacros.IsValid` _hitsoundeffect
    (:`Is Valid`
      (`GameplayStatics.PlaySound2D` _hitsoundeffect 1.0 1.0 0.0 null null))))

(fn `UserConstructionScript`
  ;[1 1 1] Set projectile movement max speed with our exposed variable.
  (bind _output_get (set `ProjectileMovementComponent.MaxSpeed` (`self.Projectile Max Speed`) (`self.ProjectileMovement`)))
  ;[1 1 1] Projectile Initial Speed setting - Handled by multiplier, set in weapons system component, clamped by Max Speed.
  (set `ProjectileMovementComponent.InitialSpeed` (`KismetMathLibrary.FClamp` (* (`self.Projectile Initial Speed`) (`self.Projectile Multiplier`)) 0.0 _output_get) (`self.ProjectileMovement`)))