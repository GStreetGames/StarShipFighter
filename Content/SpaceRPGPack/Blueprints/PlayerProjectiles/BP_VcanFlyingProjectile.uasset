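; BP_VcanFlyingProjectile is a flying player projectile Blueprint with a colored point light and hit effects.
; Its construction script runs the parent's, then tints the point light with the projectile color.
; Its clone-processing function takes a hit result, spawns the scaled hit effect system at the impact location and plays a non-spatialized 2D hit sound.
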(fn `Process Projectile Clones`
  (params (Hit :type "HitResult Structure (by ref)"))
  (`NiagaraFunctionLibrary.SpawnSystemAtLocation` (`self.Hit Effect System`) (`.Location` (`GameplayStatics.BreakHitResult` Hit)) (struct) (`self.Hit Effect Scale`))
  (`GameplayStatics.PlaySound2D` (`self.HitSoundEffect`) 1.0 1.0 0.0 null null))

(fn `UserConstructionScript`
  (`parent.UserConstructionScript`)
  (`LightComponent.SetLightColor` (`self.PointLight`) (`self.Projectile Color`) true))