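; Player-flown spaceship (FM1) with physics-based flight, extending a parent ship class.
; Each tick it applies input-driven force and torque, boosted by afterburner, and levels roll and pitch when not steered or zoomed, with pitch waiting on a mouse-idle timer.
; Camera follow and rotation-based parallax add motion feel.
; Thrust input scales the booster Niagara, glow and engine sound, while dynamic materials flash on damage and custom effects mark death and respawn.
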(event `self.Speed Updating`
  (bind _engine_sound (`self.Engine Sound`))
  (bind _dynamic_material_b (`self.Dynamic Material_B`))
  (bind _niagara (`self.Niagara`))
  (bind _returnvalue_x (`KismetMathLibrary.BreakVector` (`SceneComponent.K2_GetComponentScale` (`self.Niagara`))))
  (bind _returnvalue (+ (`|GetInputActionValue`) (`self.Afterburner Axis`)))
  (bind (_relativescale3d_x _relativescale3d_y _relativescale3d_z) (`KismetMathLibrary.BreakVector` (`SceneComponent.RelativeScale3D` _niagara)))
  ;[1 1 1] Event Speed Updating -
  (`parent.Speed Updating`)
  (`SceneComponent.SetRelativeScale3D` _niagara (`KismetMathLibrary.MakeVector` _returnvalue _relativescale3d_y _relativescale3d_z))
  (`/Engine/EditorBlueprintResources/StandardMacros.IsValid` _dynamic_material_b
    (:`Is Valid`
      (`MaterialInstanceDynamic.SetScalarParameterValue` _dynamic_material_b "Boosters Emissive Strength" (* _returnvalue 10.0)))
    (:`Is Not Valid`
      _))
  (if (> _returnvalue_x 0.9)
    (`ActorComponent.SetActive` _engine_sound true false)
    (`AudioComponent.SetVolumeMultiplier` (`self.Engine Sound`) (+ 1.0 (`self.Afterburner Axis`)))
    (else
      (`AudioComponent.FadeOut` _engine_sound 0.1 0.0 "Linear"))))

(event `self.ReceiveAnyDamage`
  (params (Damage :type "Float (single-precision)") (DamageType :type "DamageType Object Reference") (InstigatedBy :type "Controller Object Reference") (DamageCauser :type "Actor Object Reference"))
  (bind _dynamic_material (`self.Dynamic Material`))
  ;[1 1 1] Any Damage Event -
  ;;[1 1 1] Damage effect simulation
  (`MaterialInstanceDynamic.SetScalarParameterValue` _dynamic_material "Emissive Strength" 1.0)
  (`KismetSystemLibrary.Delay` 0.1)
  (`MaterialInstanceDynamic.SetScalarParameterValue` _dynamic_material "Emissive Strength" 0.0))

(event `self.ReceiveBeginPlay`
  (bind _ufo_body (`self.UFO Body`))
  (bind _ufo_body_2 (`self.UFO Body`))
  (bind _returnvalue (`PrimitiveComponent.GetMaterial` _ufo_body_2 2))
  ;[1 1 1] Event Begin Play -
  (`parent.ReceiveBeginPlay`)
  ;;[1 1 1] Set dynamic material for use with damage effect.
  (bind _returnvalue_2 (`PrimitiveComponent.CreateDynamicMaterialInstance` _ufo_body 0 (`PrimitiveComponent.GetMaterial` _ufo_body 0) "None"))
  (set `self.Dynamic Material` _returnvalue_2)
  ;;[1 1 1] If valid, set dynamic material for second element index (Boosters on default FM1)
  (`/Engine/EditorBlueprintResources/StandardMacros.IsValid` _returnvalue
    (:`Is Valid`
      (bind _returnvalue_3 (`PrimitiveComponent.CreateDynamicMaterialInstance` _ufo_body_2 2 _returnvalue "None"))
      (set `self.Dynamic Material_B` _returnvalue_3))
    (:`Is Not Valid`
      _))
  ;;[1 1 1] On Death Event -
  (add `/Game/SpaceRPGPack/Blueprints/Components/AC_Health.On Death` (`self.AC_Health`) (delegate `self.On Player Death`))
  ;;[1 1 1] Spand and attach sound for engine
  (bind _returnvalue_4 (`GameplayStatics.SpawnSoundAttached` "/Game/SpaceRPGPack/Audio/CUE/CUE_EngineRocket.CUE_EngineRocket" (`self.UFO Body`) "None" (0.0 0.0 0.0) (struct) "KeepRelativeOffset" false 1.0 1.0 0.0 null null false))
  (bind _output_get (set `self.Engine Sound` _returnvalue_4))
  (`ActorComponent.SetActive` _output_get false false))

(event `self.On Player Death`
  ;[1 1 1] Event Begin Play -
  ;;[1 1 1] On Death Event -
  (`parent.On Player Death`)
  (`/Game/SpaceRPGPack/Blueprints/Components/AC_Health.Reset` (`self.AC_Health`)))

(event `self.Custom Death Effects `
  (bind (_returnvalue_location _returnvalue_rotation _returnvalue_scale) (`KismetMathLibrary.BreakTransform` (`self.GetTransform`)))
  ;[1 1 1] Custom Death and Respawn -
  (`NiagaraFunctionLibrary.SpawnSystemAtLocation` "/Game/SpaceRPGPack/Effects/Explosions/NS_Explosion7.NS_Explosion7" _returnvalue_location _returnvalue_rotation (* _returnvalue_scale (2.0 2.0 2.0)))
  (`GameplayStatics.PlaySound2D` "/Game/SpaceRPGPack/Audio/CUE/CUE_Explode_00.CUE_Explode_00" 1.0 1.0 0.0 null null))

(event `self.Custom Respawn Effects`
  (bind (_returnvalue_location _returnvalue_rotation _returnvalue_scale) (`KismetMathLibrary.BreakTransform` (`self.GetTransform`)))
  ;[1 1 1] Custom Death and Respawn -
  (`NiagaraFunctionLibrary.SpawnSystemAtLocation` "/Game/SpaceRPGPack/Effects/NS_Resurrection.NS_Resurrection" _returnvalue_location _returnvalue_rotation (* _returnvalue_scale (2.0 2.0 2.0)))
  (`GameplayStatics.PlaySound2D` "/Game/SpaceRPGPack/Audio/CUE/CUE_PowerUP_01.CUE_PowerUP_01" 1.0 1.0 0.0 null null))

(event `self.ReceiveTick`
  (params (DeltaSeconds :type "Float (single-precision)"))
  ;[1 1 1] Event Tick -
  (`self.Follow Cam Behavior` 700.0 900.0 75.0 110.0 2.0)
  (`self.Camera Animation`)
  ;;[1 1 1] Add thrust and rotation.
  (`self.Add Thrust`)
  (`self.Add Ship Rotation`)
  (`self.Update Is Mouse Idle`)
  ;;[1 1 1] Auto Corrections
  (`self.Auto Correct Roll`)
  (`self.Auto Correct Pitch`))

(event `Set Mouse Idle`
  ;[1 1 1] Event Tick -
  (set `self.Is Mouse Idle` true))

(event `EnhancedInput|/Game/SpaceRPGPack/Input/Actions/IA_LookUp`
  (params (ActionValue :type "Float (double-precision)") (ElapsedSeconds :type "Float (double-precision)") (TriggeredSeconds :type "Float (double-precision)") (InputAction :type "InputAction Object Reference" :default "/Game/SpaceRPGPack/Input/Actions/IA_LookUp.IA_LookUp"))
  ;[1 1 1] All Movement -
  ;;[0.1441 0.004391 0.004025] Mouse Look Pitch and Yaw -
  (:`Triggered`
    (bind _output_get (set `self.Look Y Axis` ActionValue :!label _label))
    (set `self.Intentional Pitch` (> (`KismetMathLibrary.Abs` _output_get) 0.0)))
  (:`Completed`
    (goto _label)))

(event `EnhancedInput|/Game/SpaceRPGPack/Input/Actions/IA_LookRight`
  (params (ActionValue :type "Float (double-precision)") (ElapsedSeconds :type "Float (double-precision)") (TriggeredSeconds :type "Float (double-precision)") (InputAction :type "InputAction Object Reference" :default "/Game/SpaceRPGPack/Input/Actions/IA_LookRight.IA_LookRight"))
  ;[1 1 1] All Movement -
  ;;[0.1441 0.004391 0.004025] Mouse Look Pitch and Yaw -
  (:`Triggered`
    (set `self.Look X Axis` ActionValue :!label _label_2))
  (:`Completed`
    (goto _label_2)))

(event `EnhancedInput|/Game/SpaceRPGPack/Input/Actions/IA_RollRight`
  (params (ActionValue :type "Float (double-precision)") (ElapsedSeconds :type "Float (double-precision)") (TriggeredSeconds :type "Float (double-precision)") (InputAction :type "InputAction Object Reference" :default "/Game/SpaceRPGPack/Input/Actions/IA_RollRight.IA_RollRight"))
  ;[1 1 1] All Movement -
  ;;[0.1441 0.004391 0.004025] Roll Right Input -
  (:`Triggered`
    (bind _output_get (set `self.Roll Axis` (* ActionValue (`self.Roll Input Multiplier`)) :!label _label_3))
    (set `self.Intentional Roll` (> (`KismetMathLibrary.Abs` _output_get) 0.0)))
  (:`Completed`
    (goto _label_3)))

(fn `Add Ship Rotation`
  (`PrimitiveComponent.AddTorqueInRadians` (`self.UFO Body`) (* (`KismetMathLibrary.TransformDirection` (`self.GetTransform`) (`KismetMathLibrary.MakeVector` (+ (* (`self.Roll Axis`) 1.5) (* (`self.Look X Axis`) -0.25)) (* (`self.Look Y Axis`) -1.0) (`self.Look X Axis`))) (`self.Rotation Speed`)) "None" true))

(fn `Add Thrust`
  (bind _movement_speed (`self.Movement Speed`))
  (`PrimitiveComponent.AddForce` (`self.UFO Body`) (* (+ (* (`self.GetActorForwardVector`) (`|GetInputActionValue`)) (* (`self.GetActorRightVector`) (* (`|GetInputActionValue`) 0.75)) (* (`self.GetActorUpVector`) (* 0.5 (`|GetInputActionValue`)))) (`KismetMathLibrary.Lerp` _movement_speed (* _movement_speed (`self.Thrust Multiplier`)) (`self.Afterburner Axis`))) "None" true)
  (`self.ED_SpeedUpdate`))

(fn `Auto Correct Pitch`
  (bind _returnvalue (`SceneComponent.K2_GetComponentRotation` (`self.UFO Body`)))
  (if (and (not (`self.Intentional Pitch`)) (not (`self.bIs Zoomed In?`)) (`self.Is Mouse Idle`))
    (`SceneComponent.K2_SetWorldRotation` (`self.UFO Body`) (`KismetMathLibrary.RInterpTo_Constant` _returnvalue (`KismetMathLibrary.MakeRotator` (.roll _returnvalue) 0.0 (.yaw _returnvalue)) (`GameplayStatics.GetWorldDeltaSeconds`) 24.0) false false))
  (return))

(fn `Auto Correct Roll`
  (bind _returnvalue (`SceneComponent.K2_GetComponentRotation` (`self.UFO Body`)))
  (if (and (not (`self.Intentional Roll`)) (not (`self.bIs Zoomed In?`)))
    (`SceneComponent.K2_SetWorldRotation` (`self.UFO Body`) (`KismetMathLibrary.RInterpTo_Constant` _returnvalue (`KismetMathLibrary.MakeRotator` 0.0 (.pitch _returnvalue) (.yaw _returnvalue)) (`GameplayStatics.GetWorldDeltaSeconds`) 40.0) false false))
  (return))

(fn `Camera Animation`
  (bind _returnvalue (`GameplayStatics.GetWorldDeltaSeconds`))
  (bind _returnvalue_2 (`GameplayStatics.GetWorldDeltaSeconds`))
  (bind (_cam_rotator_roll _cam_rotator_pitch _cam_rotator_yaw) (`KismetMathLibrary.BreakRotator` (`self.Cam Rotator`)))
  (bind _minmax_pitchrate (`self.MinMax PitchRate`))
  (bind _minmax_yawrate (`self.MinMax YawRate`))
  (bind _returnvalue_3 (`SceneComponent.K2_GetComponentRotation` (`self.TPCamera`)))
  (set `self.Pitch Rate` (`KismetMathLibrary.FClamp` (+ (`self.Pitch Rate`) (- (.pitch _returnvalue_3) _cam_rotator_pitch)) (* _minmax_pitchrate -1.0) _minmax_pitchrate))
  (set `self.Yaw Rate` (`KismetMathLibrary.FClamp` (+ (`self.Yaw Rate`) (- (.yaw _returnvalue_3) _cam_rotator_yaw)) (* _minmax_yawrate -1.0) _minmax_yawrate))
  (set `self.Cam Rotator` _returnvalue_3)
  (bind _output_get (set `self.Pitch Parallax Offset` (`KismetMathLibrary.FInterpTo_Constant` (`self.Pitch Parallax Offset`) (`self.Pitch Rate`) _returnvalue 90.0)))
  (bind _output_get_2 (set `self.Yaw Parallax Offset` (`KismetMathLibrary.FInterpTo_Constant` (`self.Yaw Parallax Offset`) (`self.Yaw Rate`) _returnvalue 90.0)))
  (`SceneComponent.K2_SetRelativeLocationAndRotation` :`self` (`self.TPCamera`) :`NewLocation` (`KismetMathLibrary.MakeVector` 0.0 (* _output_get_2 -1.0) (* _output_get -1.0)))
  (set `self.Pitch Rate` (`KismetMathLibrary.FInterpTo_Constant` (`self.Pitch Rate`) 0.0 _returnvalue_2 90.0))
  (set `self.Yaw Rate` (`KismetMathLibrary.FInterpTo_Constant` (`self.Yaw Rate`) 0.0 _returnvalue_2 90.0)))

(fn `Mouse Idle Check`
  (returns (Output :type Boolean))
  (return (and (== (`self.GetInputAxisKeyValue`) 0.0) (== (`self.GetInputAxisKeyValue`) 0.0))))

(fn `Update Is Mouse Idle`
  (if (`self.Mouse Idle Check`)
    (if (and (not (`KismetSystemLibrary.K2_IsTimerActiveHandle` (`self.Mouse Idle Timer`))) (not (`self.Is Mouse Idle`)))
      (bind _returnvalue (`KismetSystemLibrary.K2_SetTimerDelegate` (`|CreateDelegate` :!event `Set Mouse Idle`) (`self.Mouse Idle Time`)))
      (set `self.Mouse Idle Timer` _returnvalue))
    (else
      (`KismetSystemLibrary.K2_ClearAndInvalidateTimerHandle` (`self.Mouse Idle Timer`))
      (set `self.Is Mouse Idle` false))))

(fn `UserConstructionScript`)