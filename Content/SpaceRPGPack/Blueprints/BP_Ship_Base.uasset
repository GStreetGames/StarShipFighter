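; BP_Ship_Base is the base player ship for a space RPG, handling input, cameras, collisions, death and respawn.
; Enhanced Input drives afterburner, zoom by camera switch, weapon component fire and HUD screens, with timelines feeding speed and boost displays.
; Death hides the ship, then timed respawn grants blinking invincibility, with empty effect events for children to override.
; Helper functions scale camera FOV with velocity and apply clamped speed upgrades, while hits deflect the ship and spawn sparks.
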(event `EnhancedInput|/Game/SpaceRPGPack/Input/Actions/IA_Afterburner`
  (params (ActionValue :type "Float (double-precision)") (ElapsedSeconds :type "Float (double-precision)") (TriggeredSeconds :type "Float (double-precision)") (InputAction :type "InputAction Object Reference" :default "/Game/SpaceRPGPack/Input/Actions/IA_Afterburner.IA_Afterburner"))
  ;[1 1 1] Input Controls
  ;;[0.1441 0.004391 0.004025] Afterburner -
  (:`Triggered`
    (set `self.Afterburner Axis` (`KismetMathLibrary.SelectFloat` ActionValue 0.0 (> (`|GetInputActionValue`) 0.1)) :!label _label))
  (:`Completed`
    (goto _label)))

(event `EnhancedInput|/Game/SpaceRPGPack/Input/Actions/IA_Pause`
  (params (ActionValue :type Boolean) (ElapsedSeconds :type "Float (double-precision)") (TriggeredSeconds :type "Float (double-precision)") (InputAction :type "InputAction Object Reference" :default "/Game/SpaceRPGPack/Input/Actions/IA_Pause.IA_Pause"))
  (bind _bp_hud_reference (`self.BP HUD Reference`))
  ;[1 1 1] Input Controls
  ;;[0.1441 0.004391 0.004025] Pause Event -
  (:`Started`
    (`/Engine/EditorBlueprintResources/StandardMacros.IsValid` _bp_hud_reference
      (:`Is Valid`
        (`/Game/SpaceRPGPack/Blueprints/Framework/BP_HUD.Pause Event` _bp_hud_reference)))))

(event `self.ReceiveBeginPlay`
  ;[1 1 1] Player Events -
  ;;[0.314 0.0185 0.01764] Event Begin Play -
  (bind _asbp_hud (cast `/Game/SpaceRPGPack/Blueprints/Framework/BP_HUD` (`PlayerController.GetHUD` (`GameplayStatics.GetPlayerController` 0)))
    (:`then`
      (set `self.BP HUD Reference` _asbp_hud))
    (:`CastFailed`
      _))
  (add `self.ED_SpeedUpdate` (delegate `Speed Updating`))
  ;;;[1 1 1] Enhanced Input
  (bind _asplayer_controller (cast `PlayerController` (`self.GetController`)))
  (bind _returnvalue (pcsubsystem `EnhancedInputLocalPlayerSubsystem` _asplayer_controller))
  (`/Engine/EditorBlueprintResources/StandardMacros.IsValid` _returnvalue
    (:`Is Valid`
      (`EnhancedInputSubsystemInterface.AddMappingContext` _returnvalue "/Game/SpaceRPGPack/Input/IMC_Default.IMC_Default" 0 (struct)))))

(event `Speed Updating`
  (bind _returnvalue (`|GetInputActionValue`))
  (bind _afterburner_axis (`self.Afterburner Axis`))
  ;[1 1 1] Player Events -
  ;;[0.314 0.0185 0.01764] Event Begin Play -
  ;;;[1 1 1] Speed display updating -
  (`/Engine/EditorBlueprintResources/StandardMacros.IsValid` (`self.BP HUD Reference`)
    (:`Is Valid`
      (if (!= _returnvalue 0.0)
        (bind (_direction _fillbar) (`Timeline|Speed Timeline` :`NewTime` _returnvalue :!label _label_2)
          (:`Update`
            (`/Game/SpaceRPGPack/Widgets/WBP_SpeedScreen.Update Speed` (`/Game/SpaceRPGPack/Widgets/WBP_HUD.WBP_SpeedScreen` (`/Game/SpaceRPGPack/Blueprints/Framework/BP_HUD.HUD Widget` (`self.BP HUD Reference`))) _fillbar)
            (if (!= _afterburner_axis 0.0)
              (bind (_direction_2 _fillbar_2) (`Timeline|Boost Timeline` :`NewTime` _afterburner_axis :!label _label_3)
                (:`Update`
                  (`/Game/SpaceRPGPack/Widgets/WBP_SpeedScreen.Update Boost` (`/Game/SpaceRPGPack/Widgets/WBP_HUD.WBP_SpeedScreen` (`/Game/SpaceRPGPack/Blueprints/Framework/BP_HUD.HUD Widget` (`self.BP HUD Reference`))) _fillbar_2)))
              (else
                (goto _label_3 :!via `SetNewTime`)))))
        (else
          (goto _label_2 :!via `SetNewTime`))))))

(event `EnhancedInput|/Game/SpaceRPGPack/Input/Actions/IA_WeaponScreen`
  (params (ActionValue :type Boolean) (ElapsedSeconds :type "Float (double-precision)") (TriggeredSeconds :type "Float (double-precision)") (InputAction :type "InputAction Object Reference" :default "/Game/SpaceRPGPack/Input/Actions/IA_WeaponScreen.IA_WeaponScreen"))
  (bind _bp_hud_reference (`self.BP HUD Reference`))
  ;[1 1 1] Input Controls
  ;;[0.1441 0.004391 0.004025] Weapons Screen (Inventory) -
  (:`Started`
    (`/Engine/EditorBlueprintResources/StandardMacros.IsValid` _bp_hud_reference
      (:`Is Valid`
        (`/Game/SpaceRPGPack/Blueprints/Framework/BP_HUD.Weapons Screen Event` _bp_hud_reference)))))

(event `EnhancedInput|/Game/SpaceRPGPack/Input/Actions/IA_Fire`
  (params (ActionValue :type Boolean) (ElapsedSeconds :type "Float (double-precision)") (TriggeredSeconds :type "Float (double-precision)") (InputAction :type "InputAction Object Reference" :default "/Game/SpaceRPGPack/Input/Actions/IA_Fire.IA_Fire"))
  (bind _ac_weaponsystem (`self.AC_WeaponSystem`))
  ;[1 1 1] Input Controls
  ;;[0.1441 0.004391 0.004025] InputAction Fire - Fire Weapons
  (:`Started`
    (`/Game/SpaceRPGPack/Blueprints/Components/AC_WeaponSystem.Start Fire` _ac_weaponsystem))
  (:`Completed`
    (`/Game/SpaceRPGPack/Blueprints/Components/AC_WeaponSystem.Stop Fire` _ac_weaponsystem)))

(event `On Player Death`
  (bind _ac_weaponsystem (`self.AC_WeaponSystem`))
  ;[1 1 1] Player Events -
  ;;[0.314 0.0185 0.01764] Player Death Event - Handles basic player death, respawn and continues.
  (set `self.bCanBeDamaged` false)
  (`self.DisableInput` (`GameplayStatics.GetPlayerController` 0))
  (`self.Switch Cameras` false) ; leave first person when dead!
  (`self.Custom Death Effects `)
  (`KismetSystemLibrary.Delay` 0.2)
  (`self.SetActorHiddenInGame` true)
  (`KismetSystemLibrary.Delay` 0.2)
  (`KismetSystemLibrary.K2_SetTimer` null "Respawn" (`self.Respawn Delay`))
  ;;;[1 1 1] Stop weapons fire when dead!
  (set `/Game/SpaceRPGPack/Blueprints/Components/AC_WeaponSystem.Trigger Down?` false _ac_weaponsystem)
  (`KismetSystemLibrary.K2_ClearAndInvalidateTimerHandle` (`/Game/SpaceRPGPack/Blueprints/Components/AC_WeaponSystem.Primary Fire Timer` _ac_weaponsystem)))

(event `EnhancedInput|/Game/SpaceRPGPack/Input/Actions/IA_Aim`
  (params (ActionValue :type Boolean) (ElapsedSeconds :type "Float (double-precision)") (TriggeredSeconds :type "Float (double-precision)") (InputAction :type "InputAction Object Reference" :default "/Game/SpaceRPGPack/Input/Actions/IA_Aim.IA_Aim"))
  ;[1 1 1] Input Controls
  ;;[0.1441 0.004391 0.004025] Aim Zoom -
  (:`Started`
    (bind _output_get (set `self.bIs Zoomed In?` ActionValue :!label _label_4))
    (`self.Switch Cameras` _output_get))
  (:`Completed`
    (goto _label_4)))

(event `Respawn`
  (bind _ufo_body (`self.UFO Body`))
  ;[1 1 1] Player Events -
  ;;[0.314 0.0185 0.01764] Respawn Event -
  (`self.SetActorHiddenInGame` false)
  (`self.Custom Respawn Effects`)
  (`KismetSystemLibrary.Delay` (`self.Input Delay`))
  (`self.EnableInput` (`GameplayStatics.GetPlayerController` 0))
  ;;;[1 1 1] Set the play rate for the invincibility animation timeline.
  (`TimelineComponent.SetPlayRate` (`self.Timeline_0`) (/ 1.0 (`self.Invincible Time`)))
  ;;;[1 1 1] Invincibility visual effect, then on finished reset the takes damage component, set 'Can Be Damaged' to true, and set visibility to True.
  (`Timeline|Timeline_0` :!via `PlayFromStart`
    (:`Finished`
      (set `self.bCanBeDamaged` true)
      (`SceneComponent.SetVisibility` _ufo_body true true))
    (:`Toggle Visibility`
      (`SceneComponent.ToggleVisibility` _ufo_body true))))

(event `self.ReceiveHit`
  (params (MyComp :type "PrimitiveComponent Object Reference") (Other :type "Actor Object Reference") (OtherComp :type "PrimitiveComponent Object Reference") (bSelfMoved :type Boolean) (HitLocation :type "Vector Structure") (HitNormal :type "Vector Structure") (NormalImpulse :type "Vector Structure") (Hit :type "HitResult Structure (by ref)"))
  ;[1 1 1] Player Events -
  ;;[0.314 0.0185 0.01764] Event Hit - (Effects for hitting an obstacle)
  ;;;[1 1 1] Deflect when colliding
  (`self.K2_SetActorRotation` (`KismetMathLibrary.RLerp` (`self.K2_GetActorRotation`) (`KismetMathLibrary.Conv_VectorToRotator` NormalImpulse) 0.025 true))
  (if (> (`KismetMathLibrary.VSize` (`self.GetVelocity`)) 300.0)
    (`NiagaraFunctionLibrary.SpawnSystemAtLocation` "/Game/SpaceRPGPack/Effects/NS_Hitspark.NS_Hitspark" (`.ImpactPoint` (`GameplayStatics.BreakHitResult` Hit)))))

(event `Custom Death Effects`
  ;[1 1 1] Player Events -
  ;;[0.314 0.0185 0.01764] An empty custom event to be overridden in children, to create unique death effects.
)

(event `Custom Respawn Effects`
  ;[1 1 1] Player Events -
  ;;[0.314 0.0185 0.01764] An empty custom event to be overridden in children, to create unique respawn effects.
)

(fn `Follow Cam Behavior`
  (params (InRangeA :type "Float (double-precision)") (InRangeB :type "Float (double-precision)") (OutRangeA :type "Float (double-precision)") (OutRangeB :type "Float (double-precision)") (InterpSpeed :type "Float (double-precision)"))
  (bind _tpcamera (`self.TPCamera`))
  (set `CameraComponent.FieldOfView` (`KismetMathLibrary.FInterpTo_Constant` (`CameraComponent.FieldOfView` _tpcamera) (`KismetMathLibrary.FClamp` (`KismetMathLibrary.MapRangeUnclamped` (`KismetMathLibrary.VSize` (`self.GetVelocity`)) InRangeA InRangeB OutRangeA OutRangeB) 75.0 110.0) (`GameplayStatics.GetWorldDeltaSeconds`) InterpSpeed) _tpcamera) ; Increase the camera's FOV to enhance the feeling of speed when moving fast
)

(fn `Speed Up`
  (params (`Speed Up Amount` :type "Float (double-precision)"))
  ;[0.1301 0.005605 0.2016] Speed Up - Power up the speed and boost multiplier of the ship
  (set `self.Movement Speed` (`KismetMathLibrary.FClamp` (+ (`self.Movement Speed`) `Speed Up Amount`) 0.0 8800.0))
  (set `self.Thrust Multiplier` (`KismetMathLibrary.FClamp` (+ (`self.Thrust Multiplier`) 0.2) 0.0 8.0)))

(fn `Switch Cameras`
  (params (`Is Zoomed In?` :type Boolean))
  (`ActorComponent.SetActive` (`self.FPCamera`) `Is Zoomed In?` false)
  (`ActorComponent.SetActive` (`self.TPCamera`) (not `Is Zoomed In?`) false))

(fn `UserConstructionScript`)