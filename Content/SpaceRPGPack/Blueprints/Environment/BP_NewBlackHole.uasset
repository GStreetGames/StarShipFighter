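; BP_NewBlackHole is an environment Blueprint that displays a configurable black hole effect through materials on its BlackHole component.
; The Construction Script multiplies the component's relative scale by BlackHoleSize and averages the three axes to drive the "Black Hole Size" material parameter.
; It also passes Color to the "Shift Color" vector parameter to tint the effect.
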(fn `UserConstructionScript`
  (bind (_returnvalue_x _returnvalue_y _returnvalue_z) (`KismetMathLibrary.BreakVector` (* (`SceneComponent.RelativeScale3D` (`self.Black Hole`)) (`self.Black Hole Size`))))
  ;[0.1301 0.005605 0.2016] Construction Script -
  (`MeshComponent.SetScalarParameterValueOnMaterials` (`self.Black Hole`) "Black Hole Size" (/ (+ _returnvalue_x _returnvalue_y _returnvalue_z) 3.0))
  (`MeshComponent.SetVectorParameterValueOnMaterials` (`self.Black Hole`) "Shift Color" (`KismetMathLibrary.Conv_LinearColorToVector` (`self.Color`))))