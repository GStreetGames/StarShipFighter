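; BP_MeteorField is an environment actor that scatters a random number of BP_Meteoroid actors inside a box volume on BeginPlay.
; The construction script sizes SpawnVolume from extent variables.
; Each spawn picks a random point in the bounds and a uniform integer scale, skipping placements that still collide after adjustment.
; Health comes from a random value in the size range times MinHealth, clamped, and each meteoroid is flagged FieldSpawned.
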(event `self.ReceiveBeginPlay`
  ;[0.1441 0.004391 0.004025] Event Begin Play -
  (for _ (range (+ (`KismetMathLibrary.RandomIntegerInRange` (`self.Min Spawn`) (`self.Max Spawn`)) 1))
    (`self.Spawn Meteoroid Event`)))

(event `Spawn Meteoroid Event`
  (bind _min_health (`self.Min Health`))
  (bind (_origin _boxextent) (`KismetSystemLibrary.GetComponentBounds` (`self.Spawn Volume`)))
  (bind _returnvalue (`KismetMathLibrary.RandomIntegerInRange` (`self.Min Size`) (`self.Max Size`)))
  ;[0.1441 0.004391 0.004025] Spawn Meteoroid Event -
  (`|SpawnActorFromClass` "/Game/SpaceRPGPack/Blueprints/Enemies/BP_Meteoroid.BP_Meteoroid_C" (`KismetMathLibrary.MakeTransform` (`KismetMathLibrary.RandomPointInBoundingBox` _origin _boxextent) (struct) (* (1.0 1.0 1.0) _returnvalue)) "AdjustIfPossibleButDontSpawnIfColliding" "OverrideRootScale" null (`KismetMathLibrary.FClamp` (* _returnvalue _min_health) _min_health (`self.Max Health`)) true null))

(fn `UserConstructionScript`
  (`BoxComponent.SetBoxExtent` (`self.Spawn Volume`) (`KismetMathLibrary.MakeVector` (`self.In Box Extent X`) (`self.In Box Extent Y`) (`self.In Box Extent Z`)) true))