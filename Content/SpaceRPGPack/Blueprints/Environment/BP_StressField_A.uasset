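; BP_StressField_A is a field system actor that breaks and scatters destructible geometry collections around its location.
; On BeginPlay it applies an external cluster strain field with no falloff, sized to its sphere collision component.
; It then applies a radial linear velocity from the sphere center, using a culling field to restrict the push to that same radius.
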(event `self.ReceiveBeginPlay`
  (bind _sphere_collision (`self.Sphere Collision`))
  (bind _returnvalue (`SceneComponent.K2_GetComponentLocation` _sphere_collision))
  (bind _returnvalue_2 (`RadialFalloff.SetRadialFalloff` (`self.RadialFalloff`) 80000.0 0.0 1.0 0.0 (`SphereComponent.GetScaledSphereRadius` _sphere_collision) _returnvalue "Field_FallOff_None"))
  ;[0.314 0.0185 0.01764] Event Begin Play -
  (`FieldSystemComponent.ApplyPhysicsField` (`self.FieldSystemComponent`) true "Field_ExternalClusterStrain" null _returnvalue_2)
  (`FieldSystemComponent.ApplyPhysicsField` (`self.FieldSystemComponent`) true "Field_LinearVelocity" null (`CullingField.SetCullingField` (`self.CullingField`) _returnvalue_2 (`RadialVector.SetRadialVector` (`self.RadialVector`) 1000.0 _returnvalue) "Field_Culling_Outside")))

(fn `UserConstructionScript`)