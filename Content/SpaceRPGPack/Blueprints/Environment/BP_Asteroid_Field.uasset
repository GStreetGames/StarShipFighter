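; Asteroid field actor that scatters instanced asteroids in a spherical volume around itself and makes them destructible when hit.
; Its construction script adds a hierarchical instanced mesh component per mesh in each of eight octants, with random rotation, clock-seeded scale and radius, half the placements biased to the maximum radius.
; HitAsteroid swaps a hit instance for its mapped destructible actor at the same transform, keeping the field cheap until interaction.
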(event `/Game/SpaceRPGPack/Blueprints/Framework/Interfaces/BPI_AsteroidDamage.Hit Asteroid`
  (params (`Hit Component` :type "ActorComponent Object Reference") (Index :type Integer))
  ;[0.314 0.0185 0.01764] Event Hit Asteroid -
  (bind _ashierarchical_instanced_static_mesh_component (cast `HierarchicalInstancedStaticMeshComponent` `Hit Component`))
  (bind (_value _returnvalue) (`BlueprintMapLibrary.Map_Find` (`self.Meshes Destructibles`) (`StaticMeshComponent.StaticMesh` _ashierarchical_instanced_static_mesh_component)))
  (if _returnvalue
    (`|SpawnActorFromClass` _value (`InstancedStaticMeshComponent.GetInstanceTransform` _ashierarchical_instanced_static_mesh_component Index true) "AlwaysSpawn" "OverrideRootScale" null null)
    (`InstancedStaticMeshComponent.RemoveInstance` _ashierarchical_instanced_static_mesh_component Index)))

(fn `Create Asteroid Octant`
  (params (HISMC :type "HierarchicalInstancedStaticMeshComponent Object Reference") (`X Positive` :type Boolean) (`Y Positive` :type Boolean) (`Z Positive` :type Boolean) (Scale :type "Vector2D Structure"))
  (bind (_x _y) (`KismetMathLibrary.BreakVector2D` Scale))
  (bind (_returnvalue_year _returnvalue_month _returnvalue_day _returnvalue_hour _returnvalue_minute _returnvalue_second _returnvalue_millisecond) (`KismetMathLibrary.BreakDateTime` (`KismetMathLibrary.Now`)))
  (bind _max_radius (`self.Max Radius`))
  (bind _returnvalue (* (`KismetMathLibrary.RandomFloat`) 360.0))
  (bind _returnvalue_2 (`KismetMathLibrary.RandomFloatInRangeFromStream` _x _y (`KismetMathLibrary.MakeRandomStream` (* (* _returnvalue_minute _returnvalue_second) _returnvalue_millisecond))))
  (for _ (range (+ (`self.Unique Per Octant`) 1))
    (`InstancedStaticMeshComponent.AddInstance` HISMC (`KismetMathLibrary.MakeTransform` (* (`KismetMathLibrary.ClampVectorSize` (`KismetMathLibrary.MakeVector` (`self.Select Positive` `X Positive`) (`self.Select Positive` `Y Positive`) (`self.Select Positive` `Z Positive`)) 1.0 1.0) (`KismetMathLibrary.SelectInt` (`KismetMathLibrary.RandomIntegerInRange` (`self.Min Radius`) _max_radius) _max_radius (`KismetMathLibrary.RandomBool`))) (`KismetMathLibrary.MakeRotator` _returnvalue _returnvalue _returnvalue) (`KismetMathLibrary.MakeVector` _returnvalue_2 _returnvalue_2 _returnvalue_2)) false)))

(fn `Create Asteroids`
  (for _index (range 8)
    (bind _keys (`BlueprintMapLibrary.Map_Keys` (`self.Meshes Scale`)))
    (for _array_element _keys
      (bind _returnvalue (`AddComponent|NODE_AddHierarchicalInstancedStaticMeshComponent-0`))
      (`SceneComponent.K2_AttachToComponent` _returnvalue (`self.DefaultSceneRoot`) "None" "KeepRelative" "KeepRelative" "KeepRelative" true)
      (`StaticMeshComponent.SetStaticMesh` _returnvalue _array_element)
      (`self.Create Asteroid Octant` _returnvalue (select `int` _index :`0` true :`1` true :`2` true :`3` true :`4` false :`5` false :`6` false :`7` false) (select `int` _index :`0` true :`1` true :`2` false :`3` false :`4` true :`5` true :`6` false :`7` false) (select `int` _index :`0` true :`1` false :`2` true :`3` false :`4` true :`5` false :`6` true :`7` false) (`BlueprintMapLibrary.Map_Find` (`self.Meshes Scale`) _array_element)))))

(fn `UserConstructionScript`
  (`self.Create Asteroids`))