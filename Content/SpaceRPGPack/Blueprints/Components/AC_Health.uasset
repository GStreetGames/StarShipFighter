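; Actor component that gives its owner health, optional shields, damage-type status effects and death handling.
; It binds to the owner's OnTakeAnyDamage, draining shields first and spilling overflow into health, with dispatchers announcing changes.
; At zero health it destroys the owner or calls OnDeath.
; Surviving health hits look up the damage type in a map to start timed Frozen, Burning, Stunned or Irradiated effects that broadcast on and off.
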(event `self.ReceiveBeginPlay`
  ;[0.314 0.0185 0.01764] On Begin Play -
  ;;[1 1 1] Bind event to on ANY damage, and set the health by using the "Reset" custom event.
  (bind _output_get (set `self.Owner` (`self.GetOwner`)))
  (add `Actor.OnTakeAnyDamage` _output_get (delegate `OnDamage`))
  (`self.Reset`))

(event `OnDamage`
  (params (DamagedActor :type "Actor Object Reference") (Damage :type "Float (single-precision)") (DamageType :type "DamageType Object Reference") (InstigatedBy :type "Controller Object Reference") (DamageCauser :type "Actor Object Reference"))
  ;[0.314 0.0185 0.01764] On Begin Play -
  ;;[1 1 1] On Damage -
  (`self.Handle Damage` Damage (`GameplayStatics.GetObjectClass` DamageType)))

(event `Reset`
  ;[0.314 0.0185 0.01764] Custom Events -
  ;;[1 1 1] Reset custom event - Resets the health back to the default maximum.
  (set `self.Shields` (`self.Max Shields`))
  (`self.Update Shields`)
  (set `self.Health` (`self.Max Health`))
  (`self.Update Health`))

(fn `Damage Health`
  (params (Amount :type "Float (double-precision)") (`Damage Type` :type "DamageType Class Reference"))
  (bind _output_get (set `self.Health` (`KismetMathLibrary.FClamp` (- (`self.Health`) Amount) 0.0 (`self.Max Health`))))
  (`self.Update Health`)
  (if (<= _output_get 0.0)
    (`self.Handle Death`)
    (else
      (`self.Handle Status Effect` (`local.Damage Type`)))))

(fn `Damage Shields`
  (params (Amount :type "Float (double-precision)"))
  (set `self.Shields` (`KismetMathLibrary.FClamp` (- (`self.Shields`) Amount) 0.0 (`self.Max Shields`)))
  (`self.Update Shields`))

(fn `Handle Damage`
  (params (`Damage Caused` :type "Float (double-precision)") (`Damage Type` :type "DamageType Class Reference"))
  (locals (`Difference (Local)` :type "Float (double-precision)"))
  (if (`self.Has Shield?`)
    (set `local.Difference (Local)` (- `Damage Caused` (`self.Shields`)))
    (if (> (`local.Damage Caused`) (`self.Shields`))
      (if (> (`self.Shields`) 0.0)
        (`self.Damage Shields` (`local.Damage Caused`)))
      (`self.Damage Health` (`local.Difference (Local)`) (`local.Damage Type`))
      (else
        (`self.Damage Shields` (`local.Damage Caused`))))
    (else
      (`self.Damage Health` (`local.Damage Caused`) `Damage Type`))))

(fn `Handle Death`
  (if (`self.Destroy On Death`)
    (`Actor.SetLifeSpan` (`self.Owner`) 0.1)
    (else
      (`self.On Death`))))

(fn `Handle Status Effect`
  (params (`Damage Type` :type "DamageType Class Reference (by ref)"))
  (bind (_value _returnvalue) (`BlueprintMapLibrary.Map_Find` (`self.Status Effects`) `Damage Type`))
  ;[0.1301 0.005605 0.2016] Handle Status Effect - We check if this particular damage type has an effect and pass that on to the start status effect function.
  (if _returnvalue
    (`self.Start Status Effect` (`local.Damage Type`) _value)))

(fn `Regen Health`
  (params (Amount :type "Float (double-precision)"))
  (set `self.Health` (`KismetMathLibrary.FClamp` (+ Amount (`self.Health`)) 0.0 (`self.Max Health`)))
  (`self.Update Health`))

(fn `Regen Shields`
  (params (Amount :type "Float (double-precision)"))
  (set `self.Shields` (`KismetMathLibrary.FClamp` (+ Amount (`self.Shields`)) 0.0 (`self.Max Shields`)))
  (`self.Update Shields`))

(fn `Start Status Effect`
  (params (`Damage Type` :type "DamageType Class Reference (by ref)") (`Status Effect` :type "/Game/SpaceRPGPack/Blueprints/Framework/Structures/S_StatusEffects Structure (by ref)"))
  (bind (_timer _duration _statustype) (break `/Game/SpaceRPGPack/Blueprints/Framework/Structures/S_StatusEffects` `Status Effect`))
  (bind _returnvalue (`KismetSystemLibrary.K2_SetTimerDelegate` (select `/Game/SpaceRPGPack/Blueprints/Framework/Enumerations/E_StatusEffects` _statustype :`NewEnumerator0` (`|CreateDelegate` :!event `Stop Freeze`) :`NewEnumerator1` (`|CreateDelegate` :!event `Stop Burn`) :`NewEnumerator2` (`|CreateDelegate` :!event `Stop Stun`) :`NewEnumerator3` (`|CreateDelegate` :!event `Stop Irradiation`)) _duration))
  (`BlueprintMapLibrary.Map_Add` (`self.Status Effects`) (`local.Damage Type`) (make `/Game/SpaceRPGPack/Blueprints/Framework/Structures/S_StatusEffects` _returnvalue _duration _statustype))
  (`self.On Updated Status Effect` _statustype true))

(fn `Stop Burn`
  (`self.On Updated Status Effect` "NewEnumerator1")
  (`KismetSystemLibrary.PrintString` "stopped burning"))

(fn `Stop Freeze`
  (`self.On Updated Status Effect` "NewEnumerator0")
  (`KismetSystemLibrary.PrintString` "stopped freeze"))

(fn `Stop Irradiation`
  (`self.On Updated Status Effect` "NewEnumerator3")
  (`KismetSystemLibrary.PrintString` "stopped irradiation"))

(fn `Stop Stun`
  (`self.On Updated Status Effect` "NewEnumerator2")
  (`KismetSystemLibrary.PrintString` "stopped stunned"))