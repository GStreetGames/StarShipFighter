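; AC_EnemyWeaponSystem is an actor component that makes its owning enemy shoot projectiles at the player.
; On BeginPlay it takes the owner's Arrow component as the muzzle and starts a looping timer with a randomized interval, cleared when the owner is destroyed.
; Each shot spawns an EnemyProjectile aimed at the player pawn's current location, passing color, damage, speed, range and hit settings.
; Firing also plays a 2D sound and a muzzle effect.
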(event `self.ReceiveBeginPlay`
  (set `self.Spawn Component` (`Actor.GetComponentByClass` (`self.GetOwner`) "/Script/Engine.ArrowComponent"))
  (bind _returnvalue (`KismetSystemLibrary.K2_SetTimerDelegate` (delegate `Fire`) (`KismetMathLibrary.RandomFloatInRange` 1.0 2.5) true))
  (add `Actor.OnDestroyed` (`self.GetOwner`) (delegate `Dead`)))

(event `Dead`
  (params (DestroyedActor :type "Actor Object Reference"))
  (`KismetSystemLibrary.K2_ClearAndInvalidateTimerHandle` (stale `self.ReceiveBeginPlay` _returnvalue)))

(event `Fire`
  (bind (_returnvalue_location _returnvalue_rotation _returnvalue_scale) (`KismetMathLibrary.BreakTransform` (`SceneComponent.K2_GetComponentToWorld` (`self.Spawn Component`))))
  (bind _returnvalue (`SceneComponent.K2_GetComponentLocation` (`self.Spawn Component`)))
  (`|SpawnActorFromClass` (`self.Enemy Projectile`) (`KismetMathLibrary.MakeTransform` _returnvalue (`KismetMathLibrary.Conv_VectorToRotator` (- (`Actor.K2_GetActorLocation` (`GameplayStatics.GetPlayerPawn` 0)) _returnvalue))) "AlwaysSpawn" "OverrideRootScale" (`self.GetOwner`) (`self.Projectile Color`) (`self.Projectile Color 2`) "/Game/SpaceRPGPack/Effects/Explosions/Nia/NS_BIGPULSE.NS_BIGPULSE" (`self.Hit Effect System`) (`self.Hit Sound`) (`self.Projectile Range`) (`self.Projectile Damage`) (`self.Projectile Speed`) (`self.Damage Type Class`) null)
  (`GameplayStatics.PlaySound2D` (`self.Firing Sound`) 1.0 1.0 0.0 null null) ; Firing Sound
  (`NiagaraFunctionLibrary.SpawnSystemAtLocation` (`self.Muzzle Effect System`) _returnvalue_location _returnvalue_rotation _returnvalue_scale))