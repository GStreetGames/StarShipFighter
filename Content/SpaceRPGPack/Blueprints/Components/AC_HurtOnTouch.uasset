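; AC_HurtOnTouch is an actor component that damages ships that overlap its owning actor.
; On BeginPlay it binds to the owner's begin-overlap event and reacts only to actors derived from BP_Ship_Base.
; It applies BaseDamage of the configured damage type to the ship with the owner as causer.
; When DamageSelf is set, it also deals that damage to the owner's AC_Health component, if present.
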(event `self.ReceiveBeginPlay`
  (add `Actor.OnActorBeginOverlap` (`self.GetOwner`) (delegate `Overlapping`)))

(event `Overlapping`
  (params (OverlappedActor :type "Actor Object Reference") (OtherActor :type "Actor Object Reference"))
  (bind _returnvalue (`Actor.GetComponentByClass` (`self.GetOwner`) "/Game/SpaceRPGPack/Blueprints/Components/AC_Health.AC_Health_C"))
  (bind _asbp_ship_base (cast `/Game/SpaceRPGPack/Blueprints/BP_Ship_Base` OtherActor))
  (`GameplayStatics.ApplyDamage` _asbp_ship_base (`self.Base Damage`) null OverlappedActor (`self.Damage Type Class`))
  (if (`self.Damage Self?`)
    (`/Engine/EditorBlueprintResources/StandardMacros.IsValid` _returnvalue
      (:`Is Valid`
        (`/Game/SpaceRPGPack/Blueprints/Components/AC_Health.Damage Health` _returnvalue (`self.Base Damage`) (`self.Damage Type Class`))))))