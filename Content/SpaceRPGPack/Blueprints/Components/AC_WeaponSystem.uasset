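; Actor component that runs a ship's primary and secondary weapons, collected and equipped from DT_Weapons rows.
; Tagged arrow components on the owner serve as muzzles, with cooldowns and timers driving semi-auto, burst, full-auto and charged fire.
; Each shot is either a line-trace hitscan with a Niagara beam or a spawned projectile; charged weapons hold an attached projectile until release.
; Power-ups raise a weapon power level that scales damage, range and fire rate.
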(event `Fire Primary Weapons`
  (bind _current_primary_weapon (`self.Current Primary Weapon`))
  (bind ((`FireRate_32_CD96BEC242294956DC16CF9E6C5AAABF` _firerate) (`FireType_55_2245916044FD87C5ABE76192FFC57F44` _firetype)) (break `/Game/SpaceRPGPack/Blueprints/Framework/Structures/S_Weapons` (`self.Current Primary Weapon`)))
  ;[0.1441 0.004391 0.004025] Fire Primary Weapon Custom Event -
  ;;[1 1 1] Firing Checks -
  ;;[1 1 1] Firing Sequence -
  (`|ExecutionSequence` :!label _label
    (:`then_0`
      (for _array_element (`self.Primary Weapons`)
        (if (or (`|EnumInequality` (`.FireType_55_2245916044FD87C5ABE76192FFC57F44` (break `/Game/SpaceRPGPack/Blueprints/Framework/Structures/S_Weapons` (`self.Current Primary Weapon`))) "NewEnumerator1") (`BlueprintMapLibrary.Map_Contains` (`self.Charged Projectiles`) _array_element))
          (`self.Weapon Fire` _array_element _current_primary_weapon) ; The actual firing of each individual weapon.
          (else
            (bind _returnvalue (`self.Create Projectile` _current_primary_weapon (`SceneComponent.K2_GetComponentLocation` _array_element) (`SceneComponent.K2_GetComponentRotation` _array_element)))
            (bind _asbp_charged_projectile (cast `/Game/SpaceRPGPack/Blueprints/PlayerProjectiles/Master/BP_ChargedProjectile` _returnvalue))
            (`BlueprintMapLibrary.Map_Add` (`self.Charged Projectiles`) _array_element _asbp_charged_projectile) ; Add the created charged projectile to the "Charged Projectiles" map/dictionary.
            (`Actor.K2_AttachToComponent` _asbp_charged_projectile _array_element "None" "KeepWorld" "KeepWorld" "KeepWorld" true) ; Attach the charged projectile to the target component.
          ))))
    (:`then_1`
      ;;[1 1 1] Timing and Validation -
      (switch `/Game/SpaceRPGPack/Blueprints/Framework/Enumerations/E_FireType` _firetype
        (:`NewEnumerator0`
          (`self.Start Primary Fire Cooldown`))
        (:`NewEnumerator2`
          (bind _result (`/Engine/EditorBlueprintResources/StandardMacros.IncrementInt` (`self.Burst Shot Count`))
            (:`  `
              (if (== _result (`self.Burst Shot Max Count`))
                (`KismetSystemLibrary.K2_ClearAndInvalidateTimerHandle` (`self.Primary Fire Timer`))
                (set `self.Burst Shot Count` 0)
                (`self.Start Primary Fire Cooldown`)
                (else
                  (bind _returnvalue_2 (`KismetSystemLibrary.K2_SetTimerDelegate` (`|CreateDelegate` :!event `Fire Primary Weapons`) (`self.Fire Rate Scaling` _firerate) true :!label _label_2))
                  (set `self.Primary Fire Timer` _returnvalue_2))))))
        (:`NewEnumerator3`
          (goto _label_2))))))

(event `self.ReceiveBeginPlay`
  ;[0.1441 0.004391 0.004025] Event Begin Play -
  (for _array_element (`Actor.K2_GetComponentsByClass` (`self.GetOwner`) "/Script/Engine.ArrowComponent")
    (bind _componenttags (`ActorComponent.ComponentTags` _array_element))
    (if (`KismetArrayLibrary.Array_Contains` _componenttags "Primary Weapon")
      (`KismetArrayLibrary.Array_Add` (`self.Primary Weapons`) _array_element) ; Add the Arrow Component to the "Primary Weapons" array.
      (elif (`KismetArrayLibrary.Array_Contains` _componenttags "Secondary Weapon")
        (`KismetArrayLibrary.Array_Add` (`self.Secondary Weapons`) _array_element) ; Add the Arrow Component to the "Secondary Weapons" array.
      ))))

(event `Try Fire Primary Weapons`
  ;[0.1441 0.004391 0.004025] Fire Primary Weapon Custom Event -
  ;;[1 1 1] Firing Checks -
  (if (and (not (`KismetTextLibrary.TextIsEmpty` (`.WeaponName_23_29942F94467AD7E6C12EBE9C16FDED39` (break `/Game/SpaceRPGPack/Blueprints/Framework/Structures/S_Weapons` (`self.Current Primary Weapon`))))) (`self.Can Primary Fire?`) (== (`self.Burst Shot Count`) 0))
    (goto _label)))

(event `/Game/SpaceRPGPack/Blueprints/Framework/Interfaces/BPI_Pickups.Weapon Interact`
  (params (`Data In` :type Name))
  ;[0.1441 0.004391 0.004025] Interfaces -
  ;;[1 1 1] Simple interface for assigning any weapon...
  (`self.Add To Weapons` `Data In`)
  (`self.Set Weapon Equipped` `Data In`) ; Cut if you don't want equip on collect!
)

(event `/Game/SpaceRPGPack/Blueprints/Framework/Interfaces/BPI_Pickups.Powerup Interact`
  ;[0.1441 0.004391 0.004025] Interfaces -
  ;;[1 1 1] Weapon Power upgrade Event
  (`self.Add Weapon Power`))

(event `Try Fire Secondary Weapons`
  ;[0.1441 0.004391 0.004025] Fire Secondary Weapon Custom Event -
  (if (and (not (`KismetTextLibrary.TextIsEmpty` (`.WeaponName_23_29942F94467AD7E6C12EBE9C16FDED39` (break `/Game/SpaceRPGPack/Blueprints/Framework/Structures/S_Weapons` (`self.Current Secondary Weapon`))))) (`self.Can Secondary Fire?`))
    (for _array_element (`self.Secondary Weapons`)
      (`self.Weapon Fire` _array_element (`self.Current Secondary Weapon`)))
    (`self.Start Secondary Fire Cooldown`)))

(event `Start Primary Fire Cooldown`
  ;[0.1441 0.004391 0.004025] Fire Cooldowns - For managing fire rates.
  ;;[1 1 1] Primary Fire Cooldown -
  (if (`self.Can Primary Fire?`)
    (set `self.Can Primary Fire?` false)
    (`KismetSystemLibrary.Delay` (`self.Fire Rate Scaling` (`.FireRate_32_CD96BEC242294956DC16CF9E6C5AAABF` (break `/Game/SpaceRPGPack/Blueprints/Framework/Structures/S_Weapons` (`self.Current Primary Weapon`)))))
    (set `self.Can Primary Fire?` true)
    (if (`self.Trigger Down?`)
      (`self.Try Fire Primary Weapons`))))

(event `Start Secondary Fire Cooldown`
  ;[0.1441 0.004391 0.004025] Fire Cooldowns - For managing fire rates.
  ;;[1 1 1] Secondary Fire Cooldown -
  (if (`self.Can Secondary Fire?`)
    (set `self.Can Secondary Fire?` false)
    (`KismetSystemLibrary.Delay` (`self.Fire Rate Scaling` (`.FireRate_32_CD96BEC242294956DC16CF9E6C5AAABF` (break `/Game/SpaceRPGPack/Blueprints/Framework/Structures/S_Weapons` (`self.Current Secondary Weapon`)))))
    (set `self.Can Secondary Fire?` true)
    (if (`self.Trigger Down?`)
      (`self.Try Fire Secondary Weapons`))))

(fn `Add To Weapons`
  (params (`Weapon ID` :type Name))
  (bind _returnvalue (`|GetDataTableRow` "/Game/SpaceRPGPack/Blueprints/Framework/DataTables/DT_Weapons.DT_Weapons" `Weapon ID`)
    (:`then`
      (`BlueprintMapLibrary.Map_Add` (`self.Weapons`) (`local.Weapon ID`) _returnvalue)
      (`self.ED_WeaponCollected`))))

(fn `Add Weapon Power`
  (bind _current_weapon_power (`self.Current Weapon Power`))
  (if (> (`self.Max Weapon Power`) _current_weapon_power)
    (bind _result (`/Engine/EditorBlueprintResources/StandardMacros.IncrementInt` _current_weapon_power)
      (:`  `
        (`self.ED_PowerUp` _result)))))

(fn `Create Projectile`
  (params (`Weapon Type` :type "/Game/SpaceRPGPack/Blueprints/Framework/Structures/S_Weapons Structure (by ref)") (`Spawn Location` :type "Vector Structure") (`Spawn Rotation` :type "Rotator Structure"))
  (returns (ReturnValue :type "/Game/SpaceRPGPack/Blueprints/PlayerProjectiles/Master/BP_ProjectileMaster Object Reference"))
  (bind ((`ProjectileClass_4_5BAA6D9743991927F61F93946CB585D6` _projectileclass) (`HitSound_10_6A4B57D4430242DDE5775EB67675453C` _hitsound) (`EffectSystem_52_D326E29B4F70F7CEF3D9E0960510F30F` _effectsystem) (`HitSystem_17_EAC8E68F400DEBD9126A2F91A89FE789` _hitsystem) (`IsHitscan?_41_066A3CCF46327032F424BDAAA30BAC01` _ishitscan_) (`DamageType_20_8F50C2744C12EBD6B377C990406106D2` _damagetype) (`DamageAmount_29_9D12E1BA4262623163DA4EB918EAD603` _damageamount) (`WeaponColor_46_CFFCA00942E8CE544ED6AFBDE4AA0E30` _weaponcolor) (`WeaponColor2_51_862D193C41FA3E783A33DB8F43765897` _weaponcolor2)) (break `/Game/SpaceRPGPack/Blueprints/Framework/Structures/S_Weapons` `Weapon Type`))
  ;[0.1301 0.005605 0.2016] Create Projectile Function - Used for spawning projectiles that charged weapon types utilize. Either for hitscan charge weapons to use for effect, or projectile charge weapons to deploy.
  (bind _returnvalue (`|SpawnActorFromClass` _projectileclass (`KismetMathLibrary.MakeTransform` `Spawn Location` `Spawn Rotation`) "AlwaysSpawn" "OverrideRootScale" null _weaponcolor _weaponcolor2 (`self.Set Weapon Damage` _damageamount) (select `bool` _ishitscan_ :`false` _effectsystem) _hitsystem _hitsound (`self.Current Weapon Power`) (`self.Set Weapon Range` (`self.Base Weapon Range`)) _damagetype null))
  (return _returnvalue) ; Return the spawned projectile for further use.
)

(fn `Fire Hitscan`
  (params (`Charged Projectile?` :type Boolean) (`Charged Projectile` :type "/Game/SpaceRPGPack/Blueprints/PlayerProjectiles/Master/BP_ChargedProjectile Object Reference") (`Weapon Type` :type "/Game/SpaceRPGPack/Blueprints/Framework/Structures/S_Weapons Structure") (`Weapon Origin` :type "SceneComponent Object Reference") (Hit :type "HitResult Structure"))
  (bind ((`EffectSystem_52_D326E29B4F70F7CEF3D9E0960510F30F` _effectsystem) (`HitSystem_17_EAC8E68F400DEBD9126A2F91A89FE789` _hitsystem) (`WeaponColor_46_CFFCA00942E8CE544ED6AFBDE4AA0E30` _weaponcolor) (`WeaponColor2_51_862D193C41FA3E783A33DB8F43765897` _weaponcolor2)) (break `/Game/SpaceRPGPack/Blueprints/Framework/Structures/S_Weapons` `Weapon Type`))
  (bind (_bblockinghit _binitialoverlap _time _distance _location _impactpoint _normal _impactnormal _physmat _hitactor _hitcomponent _hitbonename _bonename _hititem _elementindex _faceindex _tracestart _traceend) (`GameplayStatics.BreakHitResult` Hit))
  (bind ((`HitSound_10_6A4B57D4430242DDE5775EB67675453C` _hitsound) (`DamageType_20_8F50C2744C12EBD6B377C990406106D2` _damagetype) (`DamageAmount_29_9D12E1BA4262623163DA4EB918EAD603` _damageamount)) (break `/Game/SpaceRPGPack/Blueprints/Framework/Structures/S_Weapons` (`local.Weapon Type`)))
  (bind _returnvalue (select `bool` _bblockinghit :`false` _traceend :`true` _location))
  ;[0.1301 0.005605 0.2016] Fire Hitscan -
  (if `Charged Projectile?`
    (set `self.Charge Multiplier` (`/Game/SpaceRPGPack/Blueprints/PlayerProjectiles/Master/BP_ChargedProjectile.Charge Amount` `Charged Projectile`))
    (`Actor.K2_DestroyActor` `Charged Projectile`))
  (`self.Spawn Laser System` _effectsystem (`local.Weapon Origin`) _weaponcolor _weaponcolor2 _returnvalue _hitsystem)
  (`GameplayStatics.ApplyPointDamage` _hitactor (* (`self.Charge Multiplier`) (`self.Set Weapon Damage` _damageamount)) _tracestart (`local.Hit`) (`GameplayStatics.GetPlayerController` 0) (`self.GetOwner`) _damagetype)
  (`GameplayStatics.PlaySoundAtLocation` _hitsound _returnvalue (struct) 1.0 1.0 0.0 null null null null)
  ;;[1 1 1] Check for Asteroid Field single asteroid hit.
  (if (`KismetSystemLibrary.DoesImplementInterface` _hitactor "/Game/SpaceRPGPack/Blueprints/Framework/Interfaces/BPI_AsteroidDamage.BPI_AsteroidDamage_C")
    (message `/Game/SpaceRPGPack/Blueprints/Framework/Interfaces/BPI_AsteroidDamage.Hit Asteroid` _hitactor _hitcomponent _hititem) ; Interface Message for Asteroid Field Destruction.
  ))

(fn `Fire Projectile`
  (params (`Charged Projectile?` :type Boolean) (`Charged Projectile` :type "/Game/SpaceRPGPack/Blueprints/PlayerProjectiles/Master/BP_ChargedProjectile Object Reference") (`Weapon Type` :type "/Game/SpaceRPGPack/Blueprints/Framework/Structures/S_Weapons Structure (by ref)") (`Weapon Origin` :type "SceneComponent Object Reference"))
  (if `Charged Projectile?`
    (`Actor.K2_DetachFromActor` `Charged Projectile` "KeepWorld" "KeepWorld" "KeepWorld")
    (`/Game/SpaceRPGPack/Blueprints/PlayerProjectiles/Master/BP_ChargedProjectile.Fire` `Charged Projectile` (`local.Weapon Origin`))
    (else
      (bind _returnvalue (`self.Create Projectile` `Weapon Type` (`SceneComponent.K2_GetComponentLocation` `Weapon Origin`) (`SceneComponent.K2_GetComponentRotation` `Weapon Origin`)))
      (`/Game/SpaceRPGPack/Blueprints/PlayerProjectiles/Master/BP_ProjectileMaster.Fire` _returnvalue (`local.Weapon Origin`)))))

(fn `Fire Rate Scaling`
  (params (`Fire Rate In` :type "Float (double-precision)"))
  (returns (`Fire Rate Out` :type "Float (double-precision)"))
  (bind _current_weapon_power (`self.Current Weapon Power`))
  ;[0.1301 0.005605 0.2016] Fire Rate Scaling - Lower the fire rate based on weapon power. Has a lower limit to prevent silly fire rates!
  (return (select `bool` (and (> `Fire Rate In` 0.3) (> _current_weapon_power 1)) :`false` (`local.Fire Rate In`) :`true` (- `Fire Rate In` (* _current_weapon_power (`self.Fire Rate Reduction`))))))

(fn `Get Trace End`
  (params (Hit :type "HitResult Structure (by ref)"))
  (returns (ReturnValue :type "Vector Structure") (HitActor :type "Actor Object Reference"))
  (bind (_bblockinghit _binitialoverlap _time _distance _location _impactpoint _normal _impactnormal _physmat _hitactor _hitcomponent _hitbonename _bonename _hititem _elementindex _faceindex _tracestart _traceend) (`GameplayStatics.BreakHitResult` Hit))
  (return (select `bool` _bblockinghit :`false` _traceend :`true` _location) _hitactor))

(fn `Get Weapon Max`
  (returns (`bIs Max?` :type Boolean))
  (return (== (`self.Current Weapon Power`) (`self.Max Weapon Power`))))

(fn `Set Current Primary Weapon`
  (params (`Weapon ID` :type Name))
  (bind (_value _returnvalue) (`BlueprintMapLibrary.Map_Find` (`self.Weapons`) `Weapon ID`))
  (if _returnvalue
    (`self.Stop Fire`)
    (set `self.Current Primary Weapon ID` `Weapon ID`)
    (bind _output_get (set `self.Current Primary Weapon` _value)) ; Then we store the row data for reference.
    (`self.ED_PrimaryWeaponSet` (`.WeaponName_23_29942F94467AD7E6C12EBE9C16FDED39` (break `/Game/SpaceRPGPack/Blueprints/Framework/Structures/S_Weapons` _output_get)))
    (`KismetSystemLibrary.K2_ClearAndInvalidateTimerHandle` (`self.Primary Fire Timer`))
    (set `self.Burst Shot Count` 0)))

(fn `Set Current Secondary Weapon`
  (params (`Weapon ID` :type Name))
  (bind (_value _returnvalue) (`BlueprintMapLibrary.Map_Find` (`self.Weapons`) `Weapon ID`))
  (if _returnvalue
    (set `self.Current Secondary Weapon ID` `Weapon ID`)
    (bind _output_get (set `self.Current Secondary Weapon` _value))
    (`self.ED_SecondaryWeaponSet` (`.WeaponName_23_29942F94467AD7E6C12EBE9C16FDED39` (break `/Game/SpaceRPGPack/Blueprints/Framework/Structures/S_Weapons` _output_get)))))

(fn `Set Weapon Damage`
  (params (`Input Damage` :type "Float (double-precision)"))
  (returns (`Output Damage` :type "Float (double-precision)"))
  (return (* `Input Damage` (`self.Current Weapon Power`))))

(fn `Set Weapon Equipped`
  (params (`Weapon ID` :type Name))
  (bind _weapon_id (`local.Weapon ID`))
  (bind (_value _returnvalue) (`BlueprintMapLibrary.Map_Find` (`self.Weapons`) `Weapon ID`))
  (if _returnvalue
    (if (`.IsPrimaryType?_48_B3DAF4E1494576F5A1187EA559569D0F` (break `/Game/SpaceRPGPack/Blueprints/Framework/Structures/S_Weapons` _value))
      (`self.Set Current Primary Weapon` _weapon_id)
      (else
        (`self.Set Current Secondary Weapon` _weapon_id)))))

(fn `Set Weapon Range`
  (params (`Input Range` :type "Float (double-precision)"))
  (returns (`Output Range` :type "Float (double-precision)"))
  (return (* `Input Range` (`self.Current Weapon Power`))))

(fn `Spawn Attached Effects`
  (params (`System Used` :type "NiagaraSystem Object Reference") (`Scene Attach Component` :type "SceneComponent Object Reference") (`Color Parameter Name 1` :type Name) (`Color 1` :type "LinearColor Structure") (`Color Parameter Name 2` :type Name) (`Color 2` :type "LinearColor Structure"))
  ;[0.2167 0.02412 0.2041] Spawn Attached Effects -
  (bind _returnvalue (`NiagaraFunctionLibrary.SpawnSystemAttached` `System Used` `Scene Attach Component` "None" (0.0 0.0 0.0) (struct) "KeepRelativeOffset" true))
  (`FXSystemComponent.SetColorParameter` _returnvalue `Color Parameter Name 1` `Color 1`)
  (`FXSystemComponent.SetColorParameter` _returnvalue `Color Parameter Name 2` `Color 2`))

(fn `Spawn Laser System`
  (params (`Beam System` :type "NiagaraSystem Object Reference") (AttachToComponent :type "SceneComponent Object Reference") (`Color Parameter 1` :type "LinearColor Structure") (`Color Parameter 2` :type "LinearColor Structure") (`Hit Location` :type "Vector Structure") (`Hit System` :type "NiagaraSystem Object Reference"))
  ;[0.1301 0.005605 0.2016] Spawn Laser System - We are spawning a Niagara effect from the origin to the "LaserEnd" user value in a given Niagara System. The Niagara System does not need to be a beam/ribbon system, but it must have an end vector parameter value named "LaserEnd". A seperate hit effect must also be supplied via the "DT_Weapons" Data Table.
  ;;[1 1 1] Beam Effect, color, and end point.
  (bind _returnvalue (`NiagaraFunctionLibrary.SpawnSystemAttached` `Beam System` AttachToComponent "None" (0.0 0.0 0.0) (struct) "SnapToTarget" true))
  (`FXSystemComponent.SetColorParameter` _returnvalue "Color" `Color Parameter 1`)
  (`FXSystemComponent.SetColorParameter` _returnvalue "Color 2" `Color Parameter 2`)
  (`FXSystemComponent.SetVectorParameter` _returnvalue "LaserEnd" `Hit Location`)
  ;;[1 1 1] Hit effect and color.
  (bind _returnvalue_2 (`NiagaraFunctionLibrary.SpawnSystemAtLocation` `Hit System` `Hit Location`))
  (`FXSystemComponent.SetColorParameter` _returnvalue_2 "Color" `Color Parameter 1`)
  (`FXSystemComponent.SetColorParameter` _returnvalue_2 "Color 2" `Color Parameter 2`))

(fn `Start Fire`
  (set `self.Trigger Down?` true)
  (`self.Try Fire Primary Weapons`)
  (`self.Try Fire Secondary Weapons`))

(fn `Stop Fire`
  (bind ((`FireType_55_2245916044FD87C5ABE76192FFC57F44` _firetype)) (break `/Game/SpaceRPGPack/Blueprints/Framework/Structures/S_Weapons` (`self.Current Primary Weapon`)))
  (`|ExecutionSequence`
    (:`then_0`
      (if (and (`|EnumEquality` _firetype "NewEnumerator1") (`BlueprintMapLibrary.Map_IsNotEmpty` (`self.Charged Projectiles`)))
        (`self.Try Fire Primary Weapons`)
        (`BlueprintMapLibrary.Map_Clear` (`self.Charged Projectiles`))
        (`self.Start Primary Fire Cooldown` :!label _label)
        (elif (`|EnumEquality` _firetype "NewEnumerator3")
          (goto _label))))
    (:`then_1`
      (set `self.Trigger Down?` false)
      (if (== (`self.Burst Shot Count`) 0)
        (`KismetSystemLibrary.K2_ClearAndInvalidateTimerHandle` (`self.Primary Fire Timer`))))))

(fn `Trace Range`
  (params (`Weapon Origin` :type "SceneComponent Object Reference"))
  (returns (OutHit :type "HitResult Structure"))
  (bind _returnvalue (`SceneComponent.K2_GetComponentLocation` `Weapon Origin`))
  ;[0.1301 0.005605 0.2016] Trace Range - Trace from the target component location to the end location and return the hit result.
  (bind _outhit (`KismetSystemLibrary.LineTraceSingle` _returnvalue (+ _returnvalue (* (`KismetMathLibrary.GetForwardVector` (`SceneComponent.K2_GetComponentRotation` `Weapon Origin`)) (`self.Set Weapon Range` (`self.Base Weapon Range`)))) "TraceTypeQuery1" false (`|MakeArray` (`self.GetOwner`)) "None" true (struct :`R` 1.0 :`A` 1.0) (struct :`G` 1.0 :`A` 1.0) 0.1))
  (return _outhit))

(fn `Weapon Fire`
  (params (`Weapon Origin` :type "SceneComponent Object Reference") (`Weapon Type` :type "/Game/SpaceRPGPack/Blueprints/Framework/Structures/S_Weapons Structure"))
  (locals (Projectile :type "/Game/SpaceRPGPack/Blueprints/PlayerProjectiles/Master/BP_ProjectileMaster Object Reference") (`Damage Multiplier` :type "Float (double-precision)" :default 1.0))
  (bind ((`FireSound_9_C72E36BA44EB5789661BB7B458B39C6E` _firesound) (`MuzzleSystem_13_A8C390794E6E7D2D6A719CB5D3AD07D7` _muzzlesystem) (`EffectSystem_52_D326E29B4F70F7CEF3D9E0960510F30F` _effectsystem) (`IsHitscan?_41_066A3CCF46327032F424BDAAA30BAC01` _ishitscan_) (`WeaponColor_46_CFFCA00942E8CE544ED6AFBDE4AA0E30` _weaponcolor) (`WeaponColor2_51_862D193C41FA3E783A33DB8F43765897` _weaponcolor2)) (break `/Game/SpaceRPGPack/Blueprints/Framework/Structures/S_Weapons` `Weapon Type`))
  (bind _weapon_origin (`local.Weapon Origin`))
  (bind _weapon_origin_2 (`local.Weapon Origin`))
  (bind (_charged_projectile _returnvalue) (`self.Find Charged` _weapon_origin_2))
  (bind (_charged_projectile_2 _returnvalue_2) (`self.Find Charged` _weapon_origin))
  ;[0.2167 0.02412 0.2041] Weapon Fire -
  ;;[1 1 1] Fire Sound and Muzzle Flash
  (bind _outhit (`self.Trace Range` `Weapon Origin`)) ; We trace range in order to supply hit info to the next stage of the firing logic.
  (`GameplayStatics.PlaySound2D` _firesound 1.0 1.0 0.0 null null)
  (`/Engine/EditorBlueprintResources/StandardMacros.IsValid` _muzzlesystem
    (:`Is Valid`
      (`self.Spawn Attached Effects` _muzzlesystem (`local.Weapon Origin`) "Color" _weaponcolor "Color 2" _weaponcolor2) ; Muzzleflash System
    )
    (:`Is Not Valid`
      _))
  ;;[1 1 1] Fire Type
  (if _ishitscan_
    ;;[1 1 1] Hitscan Fire -
    (`self.Fire Hitscan` _returnvalue_2 _charged_projectile_2 (`local.Weapon Type`) _weapon_origin _outhit)
    (else
      ;;[1 1 1] Projectile Fire
      (`self.Fire Projectile` _returnvalue _charged_projectile (`local.Weapon Type`) _weapon_origin_2))))